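; Admin control panel actor that lets a player type an access password into an in-world widget.
; Entering its box switches input to game-and-UI, blends the view to a newly spawned camera and focuses the PasswordBox_UMG widget.
; The entered password goes through a server check event to the GameMode's RequestAccessMessage.
; Leaving the box disables the actor's input and returns the view to the player character.
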(event `self.ReceiveBeginPlay`)

(event `self.Box.OnComponentBeginOverlap`
  (params (OverlappedComponent :type "PrimitiveComponent Object Reference") (OtherActor :type "Actor Object Reference") (OtherComp :type "PrimitiveComponent Object Reference") (OtherBodyIndex :type Integer) (bFromSweep :type Boolean) (SweepResult :type "HitResult Structure (by ref)"))
  (`|ExecutionSequence`
    (:`then_0`
      (`WidgetBlueprintLibrary.SetInputMode_GameAndUIEx` (`GameplayStatics.GetPlayerController` 0) null "DoNotLock" false))
    (:`then_3`
      (bind _returnvalue (`|SpawnActorFromClass` "/Script/Engine.CameraActor" (`SceneComponent.K2_GetComponentToWorld` (`self.Camera`)) "Undefined" "OverrideRootScale" null null))
      (`PlayerController.SetViewTargetWithBlend` (`GameplayStatics.GetPlayerController` 0) _returnvalue 0.25 "VTBlend_Linear" 0.0 true))
    (:`then_4`
      (bind _aspassword_box_umg (cast `/Game/Games/Admin/PasswordBox_UMG` (`WidgetComponent.GetWidget` (`self.Widget`))))
      (`/Game/Games/Admin/PasswordBox_UMG.SetFocusOnKeyboard` _aspassword_box_umg)
      (add `/Game/Games/Admin/PasswordBox_UMG.PasswordEntered` _aspassword_box_umg (delegate `PasswordEntered_Event`)))))

(event `PasswordEntered_Event`
  (params (Password :type String))
  (`self.Server_CheckPassword` Password (`GameplayStatics.GetPlayerController` 0)))

(event `self.Box.OnComponentEndOverlap`
  (params (OverlappedComponent :type "PrimitiveComponent Object Reference") (OtherActor :type "Actor Object Reference") (OtherComp :type "PrimitiveComponent Object Reference") (OtherBodyIndex :type Integer))
  (`self.DisableInput` (`GameplayStatics.GetPlayerController` 0))
  (`PlayerController.SetViewTargetWithBlend` (`GameplayStatics.GetPlayerController` 0) (`GameplayStatics.GetPlayerCharacter` 0) 0.0 "VTBlend_Linear" 0.0 false))

(event `Server_CheckPassword`
  (params (Password :type String) (PlayerController :type "PlayerController Object Reference"))
  (message `/Game/Games/Admin/Admin_BPI.RequestAccess` (`GameplayStatics.GetGameMode`) Password PlayerController))

(fn `UserConstructionScript`)
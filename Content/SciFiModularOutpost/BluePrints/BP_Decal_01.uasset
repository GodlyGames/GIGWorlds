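; BP_Decal_01 is a configurable decal Blueprint from the SciFi Modular Outpost content, with color, decal choice and paint wear set per instance.
; Its construction script creates a dynamic material instance on the Decal component, then feeds DecalColor, SelectDecal and PaintWearLevel into the material's parameters.
; SelectDecal is shifted down by one for the material's selection index.
; The event graph holds no active logic.
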(fn `UserConstructionScript`
  (bind _dynamic_mat (`self.Dynamic Mat`))
  (`|ExecutionSequence`
    (:`then_0`
      ;[1 1 1] Set Customizable material on Decal Blueprint
      (bind _returnvalue (`DecalComponent.CreateDynamicMaterialInstance` (`self.Decal`)))
      (set `self.Dynamic Mat` _returnvalue)
      (`DecalComponent.SetDecalMaterial` (`self.Decal`) (`self.Dynamic Mat`)))
    (:`then_1`
      ;[1 1 1] Set Decal MAterial Parameters in Blueprint Detail panel
      (`MaterialInstanceDynamic.SetVectorParameterValue` _dynamic_mat "color" (`self.Decal Color`))
      (`MaterialInstanceDynamic.SetScalarParameterValue` _dynamic_mat "choose decal" (`KismetMathLibrary.Conv_IntToDouble` (- (`self.Select Decal`) 1)))
      (`MaterialInstanceDynamic.SetScalarParameterValue` _dynamic_mat "Wear contrast" (`self.Paint Wear Level`)))))
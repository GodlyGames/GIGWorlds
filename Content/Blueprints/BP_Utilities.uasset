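; BP_Utilities is a utility library of debug print functions for leveled, color-coded logging from Blueprints.
; Info, red info, error, start and end wrappers all feed DebugPrintFull with preset colors, labels or levels.
; DebugPrintFull filters screen and log output by DebugLevel, where intermediate levels pass errors plus exact matches only rather than being cumulative.
; Each message carries the time, context object's display name, label and value.
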(fn `Debug Print End`
  (params (EventName :type String))
  ;[1 1 1] Overloaded Debug to log ending of a blueprint
  (`self.Debug Print Full` EventName "End" (struct :`R` 0.5 :`G` 0.5 :`B` 0.5 :`A` 1.0) "NewEnumerator1"))

(fn `Debug Print Error`
  (params (Label :type String) (Value :type String))
  (locals (`Text Color` :type "LinearColor Structure" :default (struct :`B` 1.0)))
  ;[1 1 1] Overload of Debug Print
  (`self.Debug Print Full` Label Value (struct :`R` 1.0 :`A` 1.0) "NewEnumerator2" (`local.__WorldContext`)))

(fn `Debug Print Full`
  (params (Label :type String) (Value :type String) (`Text Color` :type "LinearColor Structure") (CallerDebugLevel :type "/Game/Blueprints/Data/E_DebugLevel Enum" :default "NewEnumerator0"))
  (locals (PrintToLog :type Boolean :default true) (PrintToScreen :type Boolean :default true) (Duration :type "Float (double-precision)" :default 20.0) (DebugLevel :type "/Game/Blueprints/Data/E_DebugLevel Enum" :default "NewEnumerator4"))
  (bind _returnvalue (`|EnumEquality` (`local.CallerDebugLevel`) "NewEnumerator2"))
  ;[1 1 1] Debug Print base with all variables accessable
  (switch `/Game/Blueprints/Data/E_DebugLevel` (`local.DebugLevel`)
    (:`NewEnumerator3`
      (bind _output_get (set `local.PrintToLog` false))
      (set `local.PrintToScreen` _output_get))
    (:`NewEnumerator2`
      (bind _output_get_2 (set `local.PrintToLog` _returnvalue))
      (set `local.PrintToScreen` _output_get_2))
    (:`NewEnumerator1`
      (bind _output_get_3 (set `local.PrintToLog` (or _returnvalue (`|EnumEquality` (`local.DebugLevel`) (`local.CallerDebugLevel`))) :!label _label))
      (set `local.PrintToScreen` _output_get_3))
    (:`NewEnumerator0`
      (goto _label))
    (:`NewEnumerator4`
      (bind _output_get_4 (set `local.PrintToLog` true))
      (set `local.PrintToScreen` _output_get_4)))
  (`KismetSystemLibrary.PrintString` (`local.__WorldContext`) (`KismetTextLibrary.Conv_TextToString` (`|FormatText` "{time}/{displayname}/{label}: {value}" (`KismetTextLibrary.AsTime_DateTime` (`KismetMathLibrary.Now`)) (`KismetSystemLibrary.GetDisplayName` (`local.__WorldContext`)) (`local.Label`) (`local.Value`))) (`local.PrintToScreen`) (`local.PrintToLog`) (`local.Text Color`) (`local.Duration`)))

(fn `Debug Print Info`
  (params (Label :type String) (Value :type String))
  (locals (`Text Color` :type "LinearColor Structure" :default (struct :`B` 1.0)))
  ;[1 1 1] Overload of Debug Print
  (`self.Debug Print Full` Label Value (struct :`R` 1.0 :`G` 1.0 :`B` 1.0 :`A` 1.0) "NewEnumerator0" (`local.__WorldContext`)))

(fn `Debug Print Info Red`
  (params (Label :type String) (Value :type String))
  ;[1 1 1] Overload of Debug Print
  (`self.Debug Print Full` Label Value (struct :`R` 1.0 :`A` 1.0) "NewEnumerator0" (`local.__WorldContext`)))

(fn `Debug Print Start`
  (params (EventName :type String))
  ;[1 1 1] Overloaded Debug to log starting of a blueprint
  (`self.Debug Print Full` EventName "Start" (struct :`R` 0.5 :`G` 0.5 :`B` 0.5 :`A` 1.0) "NewEnumerator1" (`local.__WorldContext`)))
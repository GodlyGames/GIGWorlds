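; Base in-world screen actor that shows a channel's cached Twitch image or random static images through a dynamic material instance.
; When powered, a looping timer re-downloads the image, using the offline texture on failure or in static-only mode.
; LoadNextImage feeds that texture and a random static fallback to the material.
; Box overlap enables input and help text for click power toggling and arrow-key image changes.
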(event `self.ReceiveBeginPlay`
  (`|ExecutionSequence`
    (:`then_0`
      (`SceneComponent.SetVisibility` (`self.NextImageMessage`) (`self.OnlyStaticImages`) false))
    (:`then_1`
      (if (`self.PowerOn`) :!label _label
        ;[1 1 1] Comment
        (`KismetSystemLibrary.K2_SetTimerDelegate` (delegate `EventReloadImage`) (`self.ReloadInSeconds`) true 1.0 1.0) ; Twitch cached image are updated every 5 minutes.
        (`KismetSystemLibrary.Delay` (`KismetMathLibrary.Conv_IntToDouble` (`KismetMathLibrary.RandomInteger` 5)))
        ;[1 1 1] Loads the latest cached image from the Twitch caching servers
        ;;[1 1 1] Bypasses downloading the image and shows a random static image.
        (if (`self.OnlyStaticImages`) :!label _label_2
          (set `self.TwitchTexture` "/Game/ImageViewer/Textures/T_Offline.T_Offline")
          (else
            (bind _texture (`AsyncTaskDownloadImage.DownloadImage` (`KismetTextLibrary.Conv_TextToString` (`|FormatText` (`self.Url Format Text`) (`self.TwitchChannelName`))))
              (:`OnSuccess`
                (set `self.TwitchTexture` _texture))
              (:`OnFail`
                (set `self.TwitchTexture` "/Game/ImageViewer/Textures/T_Offline.T_Offline")))))
        (`self.LoadNextImage`)
        (else
          ;[1 1 1] Turn On/Off the display
          (`self.PowerOff`))))))

(event `/Game/ImageViewer/Blueprints/BPI_Interactable.InteractOnOff`
  ;[1 1 1] Turn On/Off the display
  (bind _isa (`/Engine/EditorBlueprintResources/StandardMacros.FlipFlop` :!label _label_3)
    (:`A`
      _)
    (:`B`
      _))
  (set `self.PowerOn` (not _isa))
  (goto _label))

(event `EventReloadImage`
  ;[1 1 1] Loads the latest cached image from the Twitch caching servers
  (goto _label_2))

(event `self.StaticMesh.OnClicked`
  (params (TouchedComponent :type "PrimitiveComponent Object Reference") (ButtonPressed :type "Key Structure"))
  ;[1 1 1] Turn On/Off the display
  (goto _label_3))

(event `Key|Left`
  (params (Key :type "Key Structure"))
  ;[1 1 1] Next Image or Reload Web Image
  (:`Pressed`
    (`self.LoadNextImage` :!label _label_4)))

(event `Key|Right`
  (params (Key :type "Key Structure"))
  ;[1 1 1] Next Image or Reload Web Image
  (:`Pressed`
    (goto _label_4)))

(event `/Game/ImageViewer/Blueprints/BPI_Interactable.InteractNextImage`
  ;[1 1 1] Next Image or Reload Web Image
  (goto _label_4))

(event `self.Box.OnComponentBeginOverlap`
  (params (OverlappedComponent :type "PrimitiveComponent Object Reference") (OtherActor :type "Actor Object Reference") (OtherComp :type "PrimitiveComponent Object Reference") (OtherBodyIndex :type Integer) (bFromSweep :type Boolean) (SweepResult :type "HitResult Structure (by ref)"))
  (bind _returnvalue (`GameplayStatics.GetPlayerController` 0))
  ;[1 1 1] Turn On/Off Interaction - Right Arrow to force reload of the online image or load next random static image
  (set `PlayerController.bShowMouseCursor` true _returnvalue)
  (`self.EnableInput` _returnvalue)
  (bind _output_get (set `PlayerController.bEnableClickEvents` (`PlayerController.bShowMouseCursor` _returnvalue) _returnvalue :!label _label_5))
  (bind _returnvalue_2 (not (and _output_get (`self.ShowHelpText`))))
  (`SceneComponent.SetHiddenInGame` (`self.OnOffMessage`) _returnvalue_2 false)
  (`SceneComponent.SetHiddenInGame` (`self.NextImageMessage`) _returnvalue_2 false))

(event `self.Box.OnComponentEndOverlap`
  (params (OverlappedComponent :type "PrimitiveComponent Object Reference") (OtherActor :type "Actor Object Reference") (OtherComp :type "PrimitiveComponent Object Reference") (OtherBodyIndex :type Integer))
  (bind _returnvalue (`GameplayStatics.GetPlayerController` 0))
  ;[1 1 1] Turn On/Off Interaction - Right Arrow to force reload of the online image or load next random static image
  (set `PlayerController.bShowMouseCursor` false _returnvalue)
  (`self.DisableInput` _returnvalue)
  (goto _label_5))

(fn `GetRandomStaticImage`
  (returns (Output :type "Texture2D Object Reference"))
  (bind _staticimages (`self.StaticImages`))
  (return (`|GetArrayItem` _staticimages (`KismetMathLibrary.RandomInteger` (`KismetArrayLibrary.Array_Length` _staticimages)))))

(fn `LoadNextImage`
  ;[1 1 1] Sets the image to the one downloaded
  (`MaterialInstanceDynamic.SetTextureParameterValue` (`self.MI_TVScreen`) "WebImage" (`self.TwitchTexture`))
  ;[1 1 1] Sets a random image if the downloaded image is offline.
  (bind _output (`self.GetRandomStaticImage`))
  (`MaterialInstanceDynamic.SetTextureParameterValue` (`self.MI_TVScreen`) "StaticImage" _output))

(fn `PowerOff`
  ;[1 1 1] Turns off the display by setting it's texture to black.
  (`MaterialInstanceDynamic.SetTextureParameterValue` (`self.MI_TVScreen`) "WebImage" "/Game/ImageViewer/Textures/T_Offline.T_Offline")
  (`MaterialInstanceDynamic.SetTextureParameterValue` (`self.MI_TVScreen`) "StaticImage" "/Game/ImageViewer/Textures/DefaultMediaPlaneTexture.DefaultMediaPlaneTexture"))

(fn `UserConstructionScript`
  ;[1 1 1] Setup material Instance on construction.
  (bind _returnvalue (`PrimitiveComponent.CreateDynamicMaterialInstance` (`self.StaticMesh`) 1 "/Game/ImageViewer/Materials/MAT_ImageToStream.MAT_ImageToStream" "None"))
  (set `self.MI_TVScreen` _returnvalue))
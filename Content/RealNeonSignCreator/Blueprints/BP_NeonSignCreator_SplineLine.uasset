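; Neon sign tube actor that follows an editable spline and lights as On, Flicker, Flash or Off.
; The construction script creates dynamic material instances, builds a spline mesh per segment with mode-specific inner material and color, and orients end caps by tangent yaw.
; BeginPlay animates EmissiveBoost through delay loops, random for Flicker and alternating for Flash, or zeroes it for Off, which stays lit until then.
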(event `self.ReceiveBeginPlay`
  (bind _innermaterial (`self.InnerMaterial`))
  (bind _flashmaxontime (`self.FlashMaxOnTime`))
  (switch `/Game/RealNeonSignCreator/Blueprints/ENeonSignMode` (`self.NeonSignMode`)
    (:`NewEnumerator1`
      ;[1 1 1] Flicker
      (`MaterialInstanceDynamic.SetScalarParameterValue` (`self.InnerMaterialFlicker`) "EmissiveBoost" (`KismetMathLibrary.RandomFloatInRange` 0.0 (`self.EmissiveBoost`)) :!label _label)
      (`KismetSystemLibrary.Delay` (`KismetMathLibrary.RandomFloatInRange` 0.0 (`self.RandomFlickerMaxOnTime`)))
      (goto _label))
    (:`NewEnumerator2`
      ;[1 1 1] Flash
      (`MaterialInstanceDynamic.SetScalarParameterValue` _innermaterial "EmissiveBoost" 0.0 :!label _label_2)
      (`KismetSystemLibrary.Delay` _flashmaxontime)
      (`MaterialInstanceDynamic.SetScalarParameterValue` _innermaterial "EmissiveBoost" (`self.EmissiveBoost`))
      (`KismetSystemLibrary.Delay` _flashmaxontime)
      (goto _label_2))
    (:`NewEnumerator3`
      ;[1 1 1] Off
      (`MaterialInstanceDynamic.SetScalarParameterValue` (`self.InnerMaterial`) "EmissiveBoost" 0.0))))

(fn `UserConstructionScript`
  (bind _innermaterial (`self.InnerMaterial`))
  (bind _color (`self.Color`))
  (bind _innermaterialflicker (`self.InnerMaterialFlicker`))
  (bind _spline (`self.Spline`))
  (bind (_location _tangent) (`SplineComponent.GetLocationAndTangentAtSplinePoint` (`self.Spline`) 0 "Local"))
  (`|ExecutionSequence`
    (:`then_0`
      ;[1 1 1] Create Dynamic Instances of Materials
      (bind _returnvalue (`KismetMaterialLibrary.CreateDynamicMaterialInstance` "/Game/RealNeonSignCreator/Materials/MI_NeonTube_Inner.MI_NeonTube_Inner"))
      (set `self.InnerMaterial` _returnvalue)
      (bind _returnvalue_2 (`KismetMaterialLibrary.CreateDynamicMaterialInstance` "/Game/RealNeonSignCreator/Materials/MI_NeonTube_Outer.MI_NeonTube_Outer"))
      (set `self.OuterMaterial` _returnvalue_2)
      (bind _returnvalue_3 (`KismetMaterialLibrary.CreateDynamicMaterialInstance` "/Game/RealNeonSignCreator/Materials/MI_BlackInsulated.MI_BlackInsulated"))
      (set `self.InsulatedMaterial` _returnvalue_3)
      (bind _returnvalue_4 (`KismetMaterialLibrary.CreateDynamicMaterialInstance` "/Game/RealNeonSignCreator/Materials/MI_NeonTube_Inner_Flicker.MI_NeonTube_Inner_Flicker"))
      (set `self.InnerMaterialFlicker` _returnvalue_4))
    (:`then_1`
      ;[1 1 1] Create Spline Tube and Attach Caps
      (for _index (range (+ (- (`SplineComponent.GetNumberOfSplinePoints` (`self.Spline`)) 2) 1))
        (bind _returnvalue_5 (`AddComponent|NODE_AddSplineMeshComponent-0` :`bManualAttachment` true))
        (`SceneComponent.K2_AttachToComponent` _returnvalue_5 (`self.DefaultSceneRoot`) "None" "KeepRelative" "KeepRelative" "KeepRelative" true)
        (bind (_location_2 _tangent_2) (`SplineComponent.GetLocationAndTangentAtSplinePoint` _spline _index "Local"))
        (bind (_location_3 _tangent_3) (`SplineComponent.GetLocationAndTangentAtSplinePoint` _spline (+ _index 1) "Local"))
        (`SplineMeshComponent.SetStartAndEnd` _returnvalue_5 _location_2 _tangent_2 _location_3 _tangent_3 true)
        ;[1 1 1] Set Materials and Parameters based on Sign mode
        (`PrimitiveComponent.SetMaterial` _returnvalue_5 0 (`self.OuterMaterial`))
        (switch `/Game/RealNeonSignCreator/Blueprints/ENeonSignMode` (`self.NeonSignMode`)
          (:`NewEnumerator0`
            (`PrimitiveComponent.SetMaterial` _returnvalue_5 1 _innermaterial :!label _label)
            (`MaterialInstanceDynamic.SetScalarParameterValue` _innermaterial "EmissiveBoost" (`self.EmissiveBoost`)))
          (:`NewEnumerator1`
            (`PrimitiveComponent.SetMaterial` _returnvalue_5 1 _innermaterialflicker)
            (`MaterialInstanceDynamic.SetScalarParameterValue` _innermaterialflicker "EmissiveBoost" (`self.EmissiveBoost`)))
          (:`NewEnumerator2`
            (goto _label))
          (:`NewEnumerator3`
            (goto _label)))
        (`PrimitiveComponent.SetMaterial` _returnvalue_5 2 (`self.InsulatedMaterial`))
        (`MaterialInstanceDynamic.SetVectorParameterValue` _innermaterial "Color" _color)
        (`MaterialInstanceDynamic.SetVectorParameterValue` (`self.InnerMaterialFlicker`) "Color" _color))
      ;[1 1 1] Set Start and End Caps
      (`SceneComponent.K2_SetRelativeTransform` (`self.StartCap`) (`KismetMathLibrary.MakeTransform` _location (`KismetMathLibrary.MakeRotator` 0.0 0.0 (+ (.yaw (`KismetMathLibrary.Conv_VectorToRotator` _tangent)) 90.0))) false false)
      (`SceneComponent.K2_SetRelativeTransform` (`self.EndCap`) (`KismetMathLibrary.MakeTransform` _location_3 (`KismetMathLibrary.MakeRotator` 0.0 0.0 (- (.yaw (`KismetMathLibrary.Conv_VectorToRotator` _tangent_3)) 90.0))) false false))))
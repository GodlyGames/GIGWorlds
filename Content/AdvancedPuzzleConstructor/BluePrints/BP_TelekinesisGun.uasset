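; Telekinesis gun weapon that spots compatible puzzle objects, then triggers remote-controlled ones or grabs and throws grabbable ones.
; Sight traces drive spotting through BPI_ObjectControls messages; deployable objects must finish deploying before a timed physics-handle grab.
; Tick steers the held object and breaks the link when it drifts beyond a tolerance scaled by rotation rate.
; A second press charges throw impulse and blinker glow, or simply releases inside pickup areas.
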(event `/Game/AdvancedPuzzleConstructor/BluePrints/Core/BPI_Weapon.SetupWeaponModel_BPI`
  (params (WeaponModel :type "/Game/AdvancedPuzzleConstructor/BluePrints/Core/E_WeaponModel Enum" :default "NewEnumerator0")))

(event `self.ReceiveBeginPlay`
  ;[1 0.7134 0.1637] Init
  (`parent.ReceiveBeginPlay`)
  (`/Game/AdvancedPuzzleConstructor/BluePrints/Core/APC_AudioComponent.Init` (`self.APC_Audio_Grab`) null "/Game/AdvancedPuzzleConstructor/Sounds/Cue/TelekinesisGunGrabStop_Cue.TelekinesisGunGrabStop_Cue" "/Game/AdvancedPuzzleConstructor/Sounds/Cue/TelekinesisGunGrabLoop_Cue.TelekinesisGunGrabLoop_Cue" 1.0)
  (`/Game/AdvancedPuzzleConstructor/BluePrints/Core/APC_AudioComponent.Init` (`self.APC_Audio_Fire`) "/Game/AdvancedPuzzleConstructor/Sounds/Cue/TelekinesisGunStart_Cue.TelekinesisGunStart_Cue" "/Game/AdvancedPuzzleConstructor/Sounds/Cue/TelekinesisGunStop_Cue.TelekinesisGunStop_Cue" "/Game/AdvancedPuzzleConstructor/Sounds/Cue/TelekinesisGunLoop_Cue.TelekinesisGunLoop_Cue" 3.0)
  (set `self.WaitDeploy` false)
  (set `self.WaitGrab` false)
  (bind _returnvalue (`PrimitiveComponent.CreateDynamicMaterialInstance` (`self.GunMesh`) 1 null "None"))
  (set `self.DMI` _returnvalue)
  (`self.UpdateBlinker` 0.0))

(event `ProcessLastSpottedObject`
  (params (Actor :type "Actor Object Reference"))
  ;[1 1 1] Helper events for Spot / Unspot
  (`/Engine/EditorBlueprintResources/StandardMacros.IsValid` Actor
    (:`Is Valid`
      (message `/Game/AdvancedPuzzleConstructor/BluePrints/Core/BPI_ObjectControls.SpotObject_BPI` Actor false)
      (bind _indeployment (message `/Game/AdvancedPuzzleConstructor/BluePrints/Core/BPI_ObjectControls.IsDeploymentInProgress_BPI` Actor))
      (if _indeployment
        (message `/Game/AdvancedPuzzleConstructor/BluePrints/Core/BPI_ObjectControls.StartStopDeploy_BPI` Actor false)))))

(event `ProcessNewSpottedObject`
  (params (Actor :type "Actor Object Reference"))
  ;[1 1 1] Helper events for Spot / Unspot
  (message `/Game/AdvancedPuzzleConstructor/BluePrints/Core/BPI_ObjectControls.SpotObject_BPI` Actor true)
  (message `/Game/AdvancedPuzzleConstructor/BluePrints/Core/BPI_ObjectControls.SetTargetLocation_BPI` Actor (`SceneComponent.K2_GetComponentLocation` (`self.GrabTargetPoint`)))
  (`self.UpdateBlinker` (`self.MinGrabLightPower`)))

(event `ManageSoundFire`
  (params (LoopOnly :type Boolean) (StartSound :type Boolean) (StopStartSound :type Boolean))
  (bind _apc_audio_fire (`self.APC_Audio_Fire`))
  ;[1 1 1] Fire sound manager
  (if LoopOnly
    (`/Game/AdvancedPuzzleConstructor/BluePrints/Core/APC_AudioComponent.LoopOnly` (`self.APC_Audio_Fire`))
    (elif StartSound
      (`/Game/AdvancedPuzzleConstructor/BluePrints/Core/APC_AudioComponent.StartToLoop` _apc_audio_fire)
      (elif StopStartSound
        (`/Game/AdvancedPuzzleConstructor/BluePrints/Core/APC_AudioComponent.StopStartSound` _apc_audio_fire)
        (else
          (`/Game/AdvancedPuzzleConstructor/BluePrints/Core/APC_AudioComponent.LoopToEnd` _apc_audio_fire))))))

(event `ManageSoundGrab`
  (params (LoopGrabSound :type Boolean))
  (bind _apc_audio_grab (`self.APC_Audio_Grab`))
  ;[1 1 1] Grab mode sound manager
  (if LoopGrabSound
    (`/Game/AdvancedPuzzleConstructor/BluePrints/Core/APC_AudioComponent.StartToLoop` _apc_audio_grab)
    (else
      (`/Game/AdvancedPuzzleConstructor/BluePrints/Core/APC_AudioComponent.LoopToEnd` _apc_audio_grab))))

(event `UpdateArmedAnim`
  ;[1 1 1] Spot / Unspot Telekinesis object
  (bind _asbp_telekinesis_gun_anim (cast `/Game/AdvancedPuzzleConstructor/BluePrints/BP_TelekinesisGun_Anim` (`SkeletalMeshComponent.GetAnimInstance` (`self.GunMesh`)) :!label _label))
  (set `/Game/AdvancedPuzzleConstructor/BluePrints/BP_TelekinesisGun_Anim.IsArmed` (or (`self.ObjectSpotted`) (`self.ObjectGrabbed`)) _asbp_telekinesis_gun_anim))

(event `self.OnSpotted`
  (bind _lastspottedactor (`self.LastSpottedActor`))
  (bind (_bblockinghit _binitialoverlap _time _distance _location _impactpoint _normal _impactnormal _physmat _hitactor) (`GameplayStatics.BreakHitResult` (`self.TraceSightHitResult`)))
  ;[1 1 1] Spot / Unspot Telekinesis object
  (if (`KismetSystemLibrary.DoesImplementInterface` _hitactor "/Game/AdvancedPuzzleConstructor/BluePrints/Core/BPI_ObjectControls.BPI_ObjectControls_C")
    (bind _istelekinesisobject (message `/Game/AdvancedPuzzleConstructor/BluePrints/Core/BPI_ObjectControls.IsTelekinesisCompatible_BPI` _hitactor))
    (bind _result (message `/Game/AdvancedPuzzleConstructor/BluePrints/Core/BPI_ObjectControls.ObjectCanBeUsed` _hitactor))
    (if (and _result _istelekinesisobject)
      (if (not (== (`self.LastSpottedActor`) _hitactor))
        (`self.ProcessLastSpottedObject` (`self.LastSpottedActor`))
        (bind _result_2 (`self.IsObjectCanBeGrabbed` _hitactor))
        (if _result_2
          (set `self.ObjectSpotted` true)
          (set `self.LastSpottedActor` _hitactor)
          (`self.ProcessNewSpottedObject` _hitactor)
          (goto _label)
          (else
            (set `self.ObjectSpotted` false)
            (goto _label))))
      (else
        ;;[1 1 1] Switch Off spotted object
        (set `self.ObjectSpotted` false :!label _label_2)
        (`/Engine/EditorBlueprintResources/StandardMacros.IsValid` _lastspottedactor
          (:`Is Valid`
            (`self.ProcessLastSpottedObject` _lastspottedactor)
            (`/Game/AdvancedPuzzleConstructor/BluePrints/Core/APC_AudioComponent.StopAll` (`self.APC_Audio_Grab`))
            (`/Game/AdvancedPuzzleConstructor/BluePrints/Core/APC_AudioComponent.StopAll` (`self.APC_Audio_Fire`))
            (set `self.LastSpottedActor` null)
            (`self.UpdateBlinker` 0.0)
            (goto _label)))))
    (else
      (goto _label_2))))

(event `self.OffSpotted`
  ;[1 1 1] Spot / Unspot Telekinesis object
  ;;[1 1 1] Switch Off spotted object
  (goto _label_2))

(event `ReleaseObject`
  (bind _lastspottedactor (`self.LastSpottedActor`))
  ;[1 1 1] Release object. Break link with Telekinesis Gun
  (`self.UpdateBlinker` 0.0)
  (bind _indeployment (message `/Game/AdvancedPuzzleConstructor/BluePrints/Core/BPI_ObjectControls.IsDeploymentInProgress_BPI` _lastspottedactor))
  (if _indeployment
    (message `/Game/AdvancedPuzzleConstructor/BluePrints/Core/BPI_ObjectControls.StartStopDeploy_BPI` _lastspottedactor false)
    (else
      (message `/Game/AdvancedPuzzleConstructor/BluePrints/Core/BPI_ObjectControls.SetObjectGrabbed_BPI` _lastspottedactor false)
      (`PhysicsHandleComponent.ReleaseComponent` (`self.PhysicsHandle`))
      (message `/Game/AdvancedPuzzleConstructor/BluePrints/Core/BPI_ObjectControls.SetAngularDamping_BPI` _lastspottedactor (`self.ObjectAngularDamping`))
      (message `/Game/AdvancedPuzzleConstructor/BluePrints/Core/BPI_ObjectControls.EnableMeshGravity_BPI` _lastspottedactor (`self.ObjectEnableGravityAfterThrow`))
      (message `/Game/AdvancedPuzzleConstructor/BluePrints/Core/BPI_ObjectControls.SpotObject_BPI` _lastspottedactor false)))
  (`/Game/AdvancedPuzzleConstructor/BluePrints/Core/APC_AudioComponent.StopAll` (`self.APC_Audio_Fire`))
  (set `self.ObjectGrabbed` false))

(event `PlayRecoilAnim`
  ;[1 1 1] Send event Play Recoil animation to the APC controller
  (bind _apccontroller (`/Game/AdvancedPuzzleConstructor/BluePrints/Core/APC_Library.LIB_GetACPController` (`self.GetOwner`)))
  (message `/Game/AdvancedPuzzleConstructor/BluePrints/Core/BPI_PlayerInterface.PlayRecoilAnim_BPI` _apccontroller 0.75))

(event `CheckBreak`
  (bind (_bblockinghit _binitialoverlap _time _distance _location _impactpoint _normal _impactnormal _physmat _hitactor _hitcomponent) (`GameplayStatics.BreakHitResult` (`self.TraceSightHitResult`)))
  ;[1 1 1] Check if object need to brek link with Telekinesis Gun
  (`/Engine/EditorBlueprintResources/StandardMacros.IsValid` _hitactor
    (:`Is Valid`
      (bind _boxtransform (message `/Game/AdvancedPuzzleConstructor/BluePrints/Core/BPI_ObjectControls.GetBoxTransform_BPI` _hitactor))
      (bind (_forward _right _up) (message `/Game/AdvancedPuzzleConstructor/BluePrints/Core/BPI_ObjectControls.GetObjectAxis_BPI` _hitactor))
      (bind _returnvalue (- (`SceneComponent.K2_GetComponentLocation` (`self.GrabTargetPoint`)) (.location _boxtransform)))
      (if (> (`KismetMathLibrary.Sqrt` (+ (`KismetMathLibrary.MultiplyMultiply_FloatFloat` (`KismetMathLibrary.Dot_VectorVector` _right _returnvalue) 2.0) (`KismetMathLibrary.MultiplyMultiply_FloatFloat` (`KismetMathLibrary.Dot_VectorVector` _up _returnvalue) 2.0))) (* (`KismetMathLibrary.FClamp` (`self.RotationRate`) 1.0 90.0) (`self.BreakableDistance`)))
        (`self.ReleaseObject`)
        (set `self.ObjectSpotted` false)
        (`self.UpdateArmedAnim`)
        (`self.StartSightTimer`)))))

(event `UpdateBlinker`
  (params (Power :type "Float (double-precision)"))
  ;[1 1 1] Blinker
  (`MaterialInstanceDynamic.SetScalarParameterValue` (`self.DMI`) "Power" Power))

(event `TryToGrabObject`
  (bind (_bblockinghit _binitialoverlap _time _distance _location _impactpoint _normal _impactnormal _physmat _hitactor _hitcomponent) (`GameplayStatics.BreakHitResult` (`self.TraceSightHitResult`)))
  ;[1 1 1] Try to grab object
  (if (`KismetSystemLibrary.IsValid` (`self.GetAttachParentActor` _hitactor))
    (`self.K2_DetachFromActor` _hitactor "KeepWorld" "KeepWorld" "KeepWorld"))
  (message `/Game/AdvancedPuzzleConstructor/BluePrints/Core/BPI_ObjectControls.EnableMeshPhysic_BPI` _hitactor true)
  (message `/Game/AdvancedPuzzleConstructor/BluePrints/Core/BPI_ObjectControls.SetAngularDamping_BPI` _hitactor 10.0)
  (`PhysicsHandleComponent.GrabComponentAtLocation` (`self.PhysicsHandle`) _hitcomponent "None" (`SceneComponent.K2_GetComponentLocation` _hitcomponent))
  (set `self.WaitGrab` true)
  (set `self.GrabStartTime` (`KismetSystemLibrary.GetGameTimeInSeconds`))
  (`self.StopSightTimer`))

(event `/Game/AdvancedPuzzleConstructor/BluePrints/Core/BPI_Weapon.Aim_BPI`
  (params (Pressed :type Boolean))
  ;[1 1 1] Aim event
  (`parent.Aim_BPI` Pressed)
  (if (not (`self.AimMode`))
    (`/Engine/EditorBlueprintResources/StandardMacros.IsValid` (`self.LastSpottedActor`)
      (:`Is Valid`
        (`self.ReleaseObject`)
        (`self.OffSpotted`)))))

(event `GrabObject`
  ;[1 1 1] Grab Telekinesis object
  (`self.UpdateBlinker` (`self.MinGrabLightPower`))
  (message `/Game/AdvancedPuzzleConstructor/BluePrints/Core/BPI_ObjectControls.SetObjectGrabbed_BPI` (`.HitActor` (`GameplayStatics.BreakHitResult` (`self.TraceSightHitResult`))) true)
  (set `self.ObjectGrabbed` true))

(event `/Game/AdvancedPuzzleConstructor/BluePrints/Core/BPI_Weapon.Fire_BPI`
  (params (Pressed :type Boolean))
  (bind (_tracesighthitresult_bblockinghit _tracesighthitresult_binitialoverlap _tracesighthitresult_time _tracesighthitresult_distance _tracesighthitresult_location _tracesighthitresult_impactpoint _tracesighthitresult_normal _tracesighthitresult_impactnormal _tracesighthitresult_physmat _tracesighthitresult_hitactor _tracesighthitresult_hitcomponent) (`GameplayStatics.BreakHitResult` (`self.TraceSightHitResult`)))
  (bind (_tracesighthitresult_bblockinghit_2 _tracesighthitresult_binitialoverlap_2 _tracesighthitresult_time_2 _tracesighthitresult_distance_2 _tracesighthitresult_location_2 _tracesighthitresult_impactpoint_2 _tracesighthitresult_normal_2 _tracesighthitresult_impactnormal_2 _tracesighthitresult_physmat_2 _tracesighthitresult_hitactor_2) (`GameplayStatics.BreakHitResult` (`self.TraceSightHitResult`)))
  (bind (_bblockinghit _binitialoverlap _time _distance _location _impactpoint _normal _impactnormal _physmat _hitactor) (`GameplayStatics.BreakHitResult` (`self.TraceSightHitResult`)))
  ;[1 1 1] Fire event
  (if Pressed
    ;;[1 1 1] Is an object grabbed?
    (if (`self.ObjectGrabbed`)
      (bind _result (`/Engine/EditorBlueprintResources/StandardMacros.IncrementInt` (`self.FirePressCount`))
        (:`  `
          (if (== _result 2)
            (bind _inpickuparea (message `/Game/AdvancedPuzzleConstructor/BluePrints/Core/BPI_ObjectControls.IsObjectInPickupArea_BPI` _tracesighthitresult_hitactor_2))
            (if _inpickuparea
              ;;[1 1 1] If object inside of Pickup area
              (`self.ReleaseObject`)
              (`self.PlayRecoilAnim`)
              (`self.ManageSoundFire` false)
              (`self.StartSightTimer`)
              (else
                ;;[1 1 1] Start normal grab sound
                (`self.ManageSoundFire` false true)
                (set `self.FireHoldTime` 0.0))))))
      (elif (`self.ObjectSpotted`)
        (bind _objecttype (message `/Game/AdvancedPuzzleConstructor/BluePrints/Core/BPI_ObjectControls.GetObjectType_BPI` _hitactor))
        (switch `/Game/AdvancedPuzzleConstructor/BluePrints/Core/E_OverlappedObjectType` _objecttype
          (:`NewEnumerator5`
            ;;[1 1 1] If object type = Remote controlled then execute Button Pressed Interface event
            (message `/Game/AdvancedPuzzleConstructor/BluePrints/Core/BPI_ObjectControls.ButtonPressed_BPI` _hitactor))
          (:`NewEnumerator7`
            (bind (_grabvector _grabspeed _throwpower _enablegravityafterthrow) (message `/Game/AdvancedPuzzleConstructor/BluePrints/Core/BPI_ObjectControls.GetGrabbingData_BPI` _hitactor))
            (set `self.ThrowPower` _throwpower)
            (set `self.ObjectEnableGravityAfterThrow` _enablegravityafterthrow)
            (bind _angulardamping (message `/Game/AdvancedPuzzleConstructor/BluePrints/Core/BPI_ObjectControls.GetAngularDamping_BPI` _hitactor))
            (set `self.ObjectAngularDamping` _angulardamping)
            (bind _deploytime (message `/Game/AdvancedPuzzleConstructor/BluePrints/Core/BPI_ObjectControls.GetDeployTime_BPI` _hitactor))
            (if (> _deploytime 0.0)
              ;;[1 1 1] Start deploy object
              (message `/Game/AdvancedPuzzleConstructor/BluePrints/Core/BPI_ObjectControls.StartStopDeploy_BPI` _hitactor true)
              (set `self.WaitDeploy` true)
              (`self.ManageSoundGrab` true)
              (else
                ;;[1 1 1] Try to grab object
                (`self.TryToGrabObject`)
                (set `self.FirePressCount` 1)))))))
    (elif (and (>= (`self.FirePressCount`) 2) (`self.ObjectGrabbed`))
      ;;[1 1 1] Throw object. Add impuls. Break link with Telekinesis Gun
      (set `self.FirePressCount` 0)
      (`self.ReleaseObject`)
      (`PrimitiveComponent.AddImpulse` _tracesighthitresult_hitcomponent (* (`KismetMathLibrary.Normal` (- (`SceneComponent.K2_GetComponentLocation` (`self.GrabTargetPoint`)) (`SceneComponent.K2_GetComponentLocation` (`self.Muzzle`)))) (* (`self.ThrowPower`) (`self.FireHoldTime`))) "None" true)
      (`self.PlayRecoilAnim`)
      (`self.ManageSoundFire` false false true)
      (`self.ManageSoundFire` false)
      (`self.StartSightTimer`)
      (else
        ;;[1 1 1] If object in Deploy stage. Stop deploy. Stop deploy sound
        (if (`self.WaitDeploy`)
          (set `self.WaitDeploy` false)
          (message `/Game/AdvancedPuzzleConstructor/BluePrints/Core/BPI_ObjectControls.StartStopDeploy_BPI` _tracesighthitresult_hitactor false)
          (`/Game/AdvancedPuzzleConstructor/BluePrints/Core/APC_AudioComponent.StopAll` (`self.APC_Audio_Grab`)))))))

(event `self.ReceiveTick`
  (params (DeltaSeconds :type "Float (single-precision)"))
  (bind (_tracesighthitresult_bblockinghit _tracesighthitresult_binitialoverlap _tracesighthitresult_time _tracesighthitresult_distance _tracesighthitresult_location _tracesighthitresult_impactpoint _tracesighthitresult_normal _tracesighthitresult_impactnormal _tracesighthitresult_physmat _tracesighthitresult_hitactor) (`GameplayStatics.BreakHitResult` (`self.TraceSightHitResult`)))
  (bind (_tracesighthitresult_bblockinghit_2 _tracesighthitresult_binitialoverlap_2 _tracesighthitresult_time_2 _tracesighthitresult_distance_2 _tracesighthitresult_location_2 _tracesighthitresult_impactpoint_2 _tracesighthitresult_normal_2 _tracesighthitresult_impactnormal_2 _tracesighthitresult_physmat_2 _tracesighthitresult_hitactor_2) (`GameplayStatics.BreakHitResult` (`self.TraceSightHitResult`)))
  (bind (_returnvalue_roll _returnvalue_pitch _returnvalue_yaw) (`KismetMathLibrary.BreakRotator` (`KismetMathLibrary.NormalizedDeltaRotator` (`self.PrevRotation`) (`self.CurrRotation`))))
  (bind (_bblockinghit _binitialoverlap _time _distance _location _impactpoint _normal _impactnormal _physmat _hitactor) (`GameplayStatics.BreakHitResult` (`self.TraceSightHitResult`)))
  (`parent.ReceiveTick` DeltaSeconds)
  ;[1 1 1] Calculate rotation rate and setup variables
  (set `self.PrevRotation` (`self.CurrRotation`))
  (set `self.CurrRotation` (`SceneComponent.K2_GetComponentRotation` (`self.GrabTargetPoint`)))
  (set `self.RotationRate` (`KismetMathLibrary.Abs` (/ (+ (`KismetMathLibrary.Abs` _returnvalue_pitch) (`KismetMathLibrary.Abs` _returnvalue_yaw)) (`self.DeltaTime`))))
  (`|ExecutionSequence`
    (:`then_0`
      ;[1 1 1] Update Physic handle target and Object rotation
      (if (or (`self.ObjectGrabbed`) (`self.WaitGrab`))
        (message `/Game/AdvancedPuzzleConstructor/BluePrints/Core/BPI_ObjectControls.SetBoxLocation_BPI` _tracesighthitresult_hitactor_2 (`SceneComponent.K2_GetComponentLocation` (`self.GrabTargetPoint`)))
        (message `/Game/AdvancedPuzzleConstructor/BluePrints/Core/BPI_ObjectControls.SetBoxRotation_BPI` _tracesighthitresult_hitactor_2 (`KismetMathLibrary.Conv_VectorToRotator` (- (`SceneComponent.K2_GetComponentLocation` (`self.Muzzle`)) (`SceneComponent.K2_GetComponentLocation` (`self.GrabTargetPoint`)))))
        (`PhysicsHandleComponent.SetTargetLocation` (`self.PhysicsHandle`) (`SceneComponent.K2_GetComponentLocation` (`self.GrabTargetPoint`)))))
    (:`then_1`
      (if (`self.WaitGrab`)
        (`/Engine/EditorBlueprintResources/StandardMacros.IsValid` _hitactor
          (:`Is Valid`
            (bind _boxtransform (message `/Game/AdvancedPuzzleConstructor/BluePrints/Core/BPI_ObjectControls.GetBoxTransform_BPI` _hitactor))
            ;[1 1 1] Try to Grab result. If within 1 sec of time object closer to Player then it's grabbed. Otherwise - break link with TK Gun
            (if (< (`KismetMathLibrary.VSize` (- (.location _boxtransform) (`SceneComponent.K2_GetComponentLocation` (`self.GrabTargetPoint`)))) (`self.BreakableDistance`))
              (set `self.WaitGrab` false)
              (`self.GrabObject`)
              (`self.ManageSoundGrab` false)
              (`self.ManageSoundFire` true)
              (`self.PlayRecoilAnim`)
              (elif (> (- (`KismetSystemLibrary.GetGameTimeInSeconds`) (`self.GrabStartTime`)) 1.0)
                (`self.ReleaseObject`)
                (set `self.WaitGrab` false)))))))
    (:`then_2`
      (if (`self.ObjectGrabbed`)
        (`self.CheckBreak`)
        (elif (and (`self.WaitDeploy`) (`self.ObjectSpotted`))
          ;[1 1 1] Deploy complete. Start try to grab object
          (bind _deploytime (message `/Game/AdvancedPuzzleConstructor/BluePrints/Core/BPI_ObjectControls.GetDeployTime_BPI` _tracesighthitresult_hitactor))
          (if (not (> _deploytime 0.0))
            (`self.TryToGrabObject`)
            (set `self.WaitDeploy` false)
            (set `self.FirePressCount` 1)))))
    (:`then_3`
      ;[1 1 1] Update Blinker Light
      (if (and (== (`self.FirePressCount`) 2) (`self.ObjectGrabbed`))
        (set `self.FireHoldTime` (`KismetMathLibrary.FClamp` (+ (`self.FireHoldTime`) (* (`self.DeltaTime`) 1.0))))
        (`self.UpdateBlinker` (`KismetMathLibrary.Lerp` (`self.MinGrabLightPower`) (`self.MaxGrabLightPower`) (`self.FireHoldTime`)))))))

(fn `GetWeaponType_BPI`
  (returns (WeaponType :type "/Game/AdvancedPuzzleConstructor/BluePrints/Core/E_WeaponType Enum"))
  ;[1 1 1] Return Telekekinesis weapon type
  (return "NewEnumerator1"))

(fn `IsObjectCanBeGrabbed`
  (params (Actor :type "Actor Object Reference"))
  (returns (Result :type Boolean))
  ;[1 1 1] Check if object can be grabbed.
  (bind _deploytime (message `/Game/AdvancedPuzzleConstructor/BluePrints/Core/BPI_ObjectControls.GetDeployTime_BPI` Actor))
  (bind _objecttype (message `/Game/AdvancedPuzzleConstructor/BluePrints/Core/BPI_ObjectControls.GetObjectType_BPI` Actor))
  (if (or (`|EnumEquality` _objecttype "NewEnumerator5") (> _deploytime 0.0))
    (bind _forward (message `/Game/AdvancedPuzzleConstructor/BluePrints/Core/BPI_ObjectControls.GetObjectAxis_BPI` Actor))
    (return (<= (`KismetMathLibrary.DegAcos` (`KismetMathLibrary.Dot_VectorVector` (* _forward -1.0) (`SceneComponent.GetForwardVector` (`self.FireDirection`)))) (`self.MaxSpotAngle`)))
    (else
      (return true))))

(fn `UserConstructionScript`
  (`parent.UserConstructionScript`))
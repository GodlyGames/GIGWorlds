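; Game mode for a multiplayer Tag game that manages players, the "It" role, timed rounds and scoring.
; PostLogin names each player, spawns a character at a ground-traced random point plus a voice chat actor, and starts random "It" selection at two players.
; Validated tags swap roles, update PlayerState stats and restart the Standard round timer.
; Twitch chat commands trigger Lava mode or global slow and fast time dilation, gated by cooldowns.
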(event `ChangeDifficulty`
  (params (NewDifficulty :type "/Game/AntizeMenuSystem/Logics/Enum/E_Difficulty Enum" :default "NewEnumerator0"))
  ;[1 1 1] Difficulty changed (Exemple)
  (set `self.CurrentDifficulty` NewDifficulty))

(event `self.K2_PostLogin`
  (params (NewPlayer :type "PlayerController Object Reference"))
  ;[1 0.5 0] Log in process - Note this happens before BeingPlay - Setup the Local Area Chat
  (`/Game/Blueprints/BP_Utilities.Debug Print Start` "OnPostLogin")
  (set `self.NewPlayer` NewPlayer)
  (`|ExecutionSequence`
    (:`then_0`
      (bind _returnvalue (`KismetArrayLibrary.Array_AddUnique` (`self.PlayerControllers`) (`self.NewPlayer`)))
      (bind _output_get (set `self.PlayerIndex` _returnvalue))
      (bind _returnvalue_2 (`KismetTextLibrary.Conv_TextToString` (`|FormatText` "Player{number}" _output_get)))
      (`self.ChangeName` (`self.NewPlayer`) _returnvalue_2 true) ; Need to ensure this actually replicates
      (bind _asps_tag (cast `/Game/Games/Tag/PS_Tag` (`Controller.PlayerState` (`self.NewPlayer`))))
      (set `/Game/Games/Tag/PS_Tag.FriendlyName` _returnvalue_2 _asps_tag))
    (:`then_4`
      (bind _outactors (`GameplayStatics.GetAllActorsOfClass` "/Game/Games/Tag/BP_SpawnPoint.BP_SpawnPoint_C"))
      (bind _returnvalue_3 (`self.SpawnLocation` (`/Game/Games/Tag/BP_SpawnPoint.SpawnBounds` (`|GetArrayItem` _outactors))))
      (bind _output_get_2 (set `self.NewSpawnLocation` _returnvalue_3))
      (bind _returnvalue_4 (`|SpawnActorFromClass` "/Game/Games/Tag/BP_TagCharacter.BP_TagCharacter_C" _output_get_2 "AdjustIfPossibleButAlwaysSpawn" "OverrideRootScale" null false null))
      (`Controller.Possess` (`self.NewPlayer`) _returnvalue_4))
    (:`then_10`
      ;;[1 1 1] Starts then game when there are atleast 2 players.
      (if (== (`self.PlayerIndex`) 1)
        (`self.Cycle Tag`)))
    (:`then_15`
      (`|SpawnActorFromClass` "/Script/UniversalVoiceChatPro.PlayerVoiceChatActor" (`self.NewSpawnLocation`) "Undefined" "OverrideRootScale" (`self.NewPlayer`) (`GameplayStatics.GetPlayerControllerID` (`self.NewPlayer`)) "" false false false 1000.0 null))))

(event `StartTagRoundTimer`
  ;[1 0.5 0] Start Round Timer
  (if (`KismetSystemLibrary.K2_IsValidTimerHandle` (`self.TagTimerHandle`))
    (`KismetSystemLibrary.K2_ClearAndInvalidateTimerHandle` (`self.TagTimerHandle`)))
  (bind _returnvalue (`KismetSystemLibrary.K2_SetTimerDelegate` (delegate `Cycle Tag`) (`self.GameRoundTimeSpan`)))
  (bind _output_get (set `self.TagTimerHandle` _returnvalue))
  (`self.TagRoundTimeReset` (`self.CalcSecondsForRoundEnd` _output_get))
  (set `self.GameType` "NewEnumerator0")
  (`self.GameTypeChange` "NewEnumerator0"))

(event `Cycle Tag`
  ;[1 0.5 0] Cycle through players and select the next "It"
  (`|ExecutionSequence`
    (:`then_0`
      (for _array_element (`self.PlayerControllers`)
        (message `/Game/Games/Tag/BPI_Tag.NotIt` _array_element)))
    (:`then_4`
      (if (>= (`KismetArrayLibrary.Array_Length` (`self.PlayerControllers`)) 2)
        (message `/Game/Games/Tag/BPI_Tag.YourIt` (`KismetArrayLibrary.Array_Random` (`self.PlayerControllers`)) "NewEnumerator0")))
    (:`then_8`
      (`self.StartTagRoundTimer`))))

(event `self.K2_OnLogout`
  (params (ExitingController :type "Controller Object Reference"))
  ;[1 0.5 0] Log out process
  (bind _asplayer_controller (cast `PlayerController` ExitingController))
  (`KismetArrayLibrary.Array_RemoveItem` (`self.PlayerControllers`) _asplayer_controller)
  (bind _isit (message `/Game/Games/Tag/BPI_Tag.CheckIt` _asplayer_controller))
  (if _isit
    (`self.StartTagRoundTimer`)))

(event `PlayerTagged`
  (params (TaggedBy :type "/Game/Games/Tag/PC_Tag Object Reference") (TaggedPlayer :type "/Game/Games/Tag/PC_Tag Object Reference") (TagType :type "/Game/Games/Tag/E_TagType Enum" :default "NewEnumerator0"))
  ;[1 0.5 0] Player Tagged
  (bind _output_get (set `self.Tagged By` TaggedBy))
  (set `self.Tagged Player` TaggedPlayer)
  (set `self.Tag Type` TagType)
  (`self.CanTag` _output_get TaggedPlayer
    (:`true`
      (`|ExecutionSequence`
        (:`then_0`
          (bind _asps_tag (cast `/Game/Games/Tag/PS_Tag` (`Controller.PlayerState` (`self.Tagged Player`))))
          (set `self.TaggedPlayerState` _asps_tag)
          (message `/Game/Games/Tag/BPI_Tag.YourIt` (`self.Tagged Player`) (`self.Tag Type`)))
        (:`then_5`
          (`/Engine/EditorBlueprintResources/StandardMacros.IsValid` (`self.Tagged By`)
            (:`Is Valid`
              (`|ExecutionSequence`
                (:`then_0`
                  (bind _asps_tag_2 (cast `/Game/Games/Tag/PS_Tag` (`Controller.PlayerState` (`self.Tagged By`))))
                  (set `self.TaggedByState` _asps_tag_2)
                  (message `/Game/Games/Tag/BPI_Tag.NotIt` (`self.Tagged By`)))
                (:`then_4`
                  (`KismetArrayLibrary.Array_Add` (`/Game/Games/Tag/PS_Tag.PlayerTagged` (`self.TaggedByState`)) (`/Game/Games/Tag/PS_Tag.FriendlyName` (`self.TaggedPlayerState`))))
                (:`then_8`
                  (set `/Game/Games/Tag/PS_Tag.TotalTimeTagged` (+ (`/Game/Games/Tag/PS_Tag.TotalTimeTagged` (`self.TaggedByState`)) (`self.RoundTimeElasped`)) (`self.TaggedByState`)))
                (:`then_13`
                  (`KismetArrayLibrary.Array_Add` (`/Game/Games/Tag/PS_Tag.PlayerTagged` (`self.TaggedPlayerState`)) (`/Game/Games/Tag/PS_Tag.FriendlyName` (`self.TaggedByState`))))
                (:`then_18`
                  (bind _result (`/Engine/EditorBlueprintResources/StandardMacros.IncrementInt` (`/Game/Games/Tag/PS_Tag.PlayerScore` (`self.TaggedByState`)))
                    (:`  `
                      (set `/Game/Games/Tag/PS_Tag.PlayerScore` _result (`self.TaggedByState`)))))))))
        (:`then_9`
          (switch `/Game/Games/Tag/E_TagType` (`self.GameType`)
            (:`NewEnumerator0`
              (`self.StartTagRoundTimer`))))))
    (:`false`
      (`/Game/Blueprints/BP_Utilities.Debug Print Info` "Tag Condition" "False"))))

(event `self.ReceiveBeginPlay`
  ;[1 0.5 0] Connect to Twitch Channel
  (`self.ConnectToTwitchChannel` "missionarygamer"))

(event `ConnectToTwitchChannel`
  (params (ChannelName :type String))
  ;[1 0.5 0] Connect to Twitch Channel
  (if (`TwitchSubsystem.JoinChannel` (subsystem `TwitchSubsystem`) ChannelName)
    (add `TwitchSubsystem.OnMessageReceived` (subsystem `TwitchSubsystem`) (delegate `OnMessageReceived_Event`))))

(event `/Game/Games/Tag/BPI_Tag.Lava`
  ;[1 0.5 0] Connect to Twitch Channel
  (if (not (`self.LavaCooldown`)) :!label _label
    (set `self.GameType` "NewEnumerator1")
    (`self.GameTypeChange` "NewEnumerator1")
    (`KismetSystemLibrary.K2_SetTimerDelegate` (delegate `ResetLavaCooldown`) 30.0)
    (set `self.LavaCooldown` true)))

(event `OnMessageReceived_Event`
  (params (ChannelName :type String) (DisplayName :type String) (MessageText :type String))
  ;[1 0.5 0] Connect to Twitch Channel
  (`/Game/Blueprints/BP_Utilities.Debug Print Info` DisplayName MessageText)
  (switch `string` MessageText
    (:`!lava`
      (goto _label))
    (:`!slowmo`
      (if (not (`self.TimeDilationCooldown`)) :!label _label_2
        (`GameplayStatics.SetGlobalTimeDilation` 0.25)
        (`KismetSystemLibrary.K2_SetTimerDelegate` (delegate `ResetTime`) (* 10.0 (`GameplayStatics.GetGlobalTimeDilation`)) :!label _label_3)
        (set `self.TimeDilationCooldown` true)))
    (:`!fastmo`
      (if (not (`self.TimeDilationCooldown`)) :!label _label_4
        (`GameplayStatics.SetGlobalTimeDilation` 2.0)
        (goto _label_3)))))

(event `ResetLavaCooldown`
  ;[1 0.5 0] Connect to Twitch Channel
  (set `self.LavaCooldown` false))

(event `/Game/Games/Tag/BPI_Tag.SlowMo`
  ;[1 0.5 0] Connect to Twitch Channel
  (goto _label_2))

(event `ResetTime`
  ;[1 0.5 0] Connect to Twitch Channel
  (`GameplayStatics.SetGlobalTimeDilation` 1.0)
  (`KismetSystemLibrary.Delay` 30.0)
  (set `self.TimeDilationCooldown` false))

(event `/Game/Games/Tag/BPI_Tag.FastMo`
  ;[1 0.5 0] Connect to Twitch Channel
  (goto _label_4))

(fn `CheckIt`
  (returns (IsIt :type Boolean))
  (return false))

(fn `SpawnLocation`
  (params (BoundingBox :type "SceneComponent Object Reference"))
  (returns (ReturnValue :type "Transform Structure"))
  (bind (_origin _boxextent) (`KismetSystemLibrary.GetComponentBounds` BoundingBox))
  (bind _returnvalue (`KismetMathLibrary.MakeVector` (.x (`KismetMathLibrary.RandomPointInBoundingBox` _origin _boxextent)) (.y (`KismetMathLibrary.RandomPointInBoundingBox` _origin _boxextent)) (+ (.z (`KismetMathLibrary.RandomPointInBoundingBox` _origin _boxextent)) 10000.0)))
  ;[1 0.5 0] Server Side
  ;;[1 1 1] Use a Line Trace to make sure the new character lands on the ground
  (bind _outhit (`KismetSystemLibrary.LineTraceSingleForObjects` :`Start` _returnvalue :`End` (+ _returnvalue (* (* (`self.GetActorUpVector`) -1) 15000.0)) :`ObjectTypes` (`|MakeArray` "ObjectTypeQuery1" :!type "EObjectTypeQuery Enum") :`DrawDebugType` "ForDuration" :`DrawTime` 2.0))
  (return (`KismetMathLibrary.MakeTransform` (`KismetMathLibrary.MakeVector` (.x (`.Location` (`GameplayStatics.BreakHitResult` _outhit))) (.y (`.Location` (`GameplayStatics.BreakHitResult` _outhit))) (+ (.z (`.Location` (`GameplayStatics.BreakHitResult` _outhit))) 1500.0)) (struct) (`self.PlayerScale`))))

(fn `UserConstructionScript`)
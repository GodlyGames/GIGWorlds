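; Sci-fi outpost gate actor with two blast doors that open and close automatically as things enter and leave their trigger boxes.
; Each box plays its own timeline on begin overlap and reverses it on end overlap, with no check on the overlapping actor.
; The timelines drive the relative Z of each door's upper and lower halves, while X and Y stay at hard-coded offsets.
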(event `self.Box.OnComponentBeginOverlap`
  (params (OverlappedComponent :type "PrimitiveComponent Object Reference") (OtherActor :type "Actor Object Reference") (OtherComp :type "PrimitiveComponent Object Reference") (OtherBodyIndex :type Integer) (bFromSweep :type Boolean) (SweepResult :type "HitResult Structure (by ref)"))
  ;[1 1 1] Blast Door 1 opening and Closing Animation
  (bind (_direction _lower _upper) (`Timeline|Gate1 open` :!label _label)
    (:`Update`
      (`SceneComponent.K2_SetRelativeLocation` (`self.Gate_01_Lower`) (`KismetMathLibrary.MakeVector` -18.031982 -209.087738 _lower) false false)
      (`SceneComponent.K2_SetRelativeLocation` (`self.Gate_01_Upper`) (`KismetMathLibrary.MakeVector` -18.959229 -209.087952 _upper) false false))))

(event `self.Box.OnComponentEndOverlap`
  (params (OverlappedComponent :type "PrimitiveComponent Object Reference") (OtherActor :type "Actor Object Reference") (OtherComp :type "PrimitiveComponent Object Reference") (OtherBodyIndex :type Integer))
  ;[1 1 1] Blast Door 1 opening and Closing Animation
  (goto _label :!via `Reverse`))

(event `self.Box1.OnComponentBeginOverlap`
  (params (OverlappedComponent :type "PrimitiveComponent Object Reference") (OtherActor :type "Actor Object Reference") (OtherComp :type "PrimitiveComponent Object Reference") (OtherBodyIndex :type Integer) (bFromSweep :type Boolean) (SweepResult :type "HitResult Structure (by ref)"))
  ;[1 1 1] Blast Door 2 opening and Closing Animation
  (bind (_direction _lower _upper) (`Timeline|Gate_02` :!label _label_2)
    (:`Update`
      (`SceneComponent.K2_SetRelativeLocation` (`self.Gate_02_Lower`) (`KismetMathLibrary.MakeVector` -18.031982 227.512207 _lower) false false)
      (`SceneComponent.K2_SetRelativeLocation` (`self.Gate_02_Upper`) (`KismetMathLibrary.MakeVector` -18.959229 227.512695 _upper) false false))))

(event `self.Box1.OnComponentEndOverlap`
  (params (OverlappedComponent :type "PrimitiveComponent Object Reference") (OtherActor :type "Actor Object Reference") (OtherComp :type "PrimitiveComponent Object Reference") (OtherBodyIndex :type Integer))
  ;[1 1 1] Blast Door 2 opening and Closing Animation
  (goto _label_2 :!via `Reverse`))

(fn `UserConstructionScript`)
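; Spline-driven pipe Blueprint for a modular sci-fi outpost that builds a run of deformed pipe meshes along an editable spline.
; The Construction Script divides the spline into whole sections sized by forward axis length times actor X scale, adding one spline mesh component per section.
; Each segment takes local positions and tangents from the spline, with tangents clamped to section length, and receives the assigned material.
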(fn `UserConstructionScript`
  (bind _returnvalue_x (`KismetMathLibrary.BreakVector` (`self.GetActorScale3D`)))
  (bind _sectionlength (`self.SectionLength`))
  (bind _sectionlength_2 (`self.SectionLength`))
  (bind _returnvalue (* (`self.Current Index`) (`self.SectionLength`)))
  (bind _returnvalue_2 (* (+ (`self.Current Index`) 1) (`self.SectionLength`)))
  (bind (_min _max) (break `Box` (`StaticMesh.GetBoundingBox` (`StaticMeshComponent.StaticMesh` (`self.Spline mesh Comp`)))))
  ;[1 1 1] Set Forward Axis
  (set `self.SectionLength` (* _returnvalue_x (`self.Forward Axis Length`)))
  ;[1 1 1] Spline Length
  (for _index (range (`KismetMathLibrary.FTrunc` (/ (`SplineComponent.GetSplineLength` (`self.Spline`)) (`self.SectionLength`))))
    (set `self.Current Index` _index)
    ;[1 1 1] Add Mesh
    (bind _returnvalue_3 (`AddComponent|NODE_AddSplineMeshComponent-2`))
    (set `self.Spline mesh Comp` _returnvalue_3)
    (set `self.Mesh Length` (- (.x _max) (.x _min)))
    ;[1 1 1] Set Start/End Position
    (`SplineMeshComponent.SetStartAndEnd` (`self.Spline mesh Comp`) (`SplineComponent.GetLocationAtDistanceAlongSpline` (`self.Spline`) _returnvalue "Local") (`KismetMathLibrary.ClampVectorSize` (`SplineComponent.GetTangentAtDistanceAlongSpline` (`self.Spline`) _returnvalue "Local") _sectionlength_2 _sectionlength_2) (`SplineComponent.GetLocationAtDistanceAlongSpline` (`self.Spline`) _returnvalue_2 "Local") (`KismetMathLibrary.ClampVectorSize` (`SplineComponent.GetTangentAtDistanceAlongSpline` (`self.Spline`) _returnvalue_2 "Local") _sectionlength _sectionlength) true)
    ;[1 1 1] Set Material
    (`PrimitiveComponent.SetMaterial` (`self.Spline mesh Comp`) 0 (`self.Material`))))
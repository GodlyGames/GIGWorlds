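; Neon sign actor that spells a Text string from per-character tube meshes and can flicker, flash or be switched off.
; The construction script looks up each character in CharToMesh, spawns spaced mesh components and applies shared dynamic materials with color and glow.
; In Flicker mode, a seeded stream picks one character for a separate flicker material.
; BeginPlay drives EmissiveBoost by mode: random flicker, timed whole-sign blinking, or zero for off.
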(event `self.ReceiveBeginPlay`
  (bind _flashmaxontime (`self.FlashMaxOnTime`))
  (bind _innermaterial (`self.InnerMaterial`))
  (switch `/Game/RealNeonSignCreator/Blueprints/ENeonSignMode` (`self.NeonSignMode`)
    (:`NewEnumerator1`
      ;[1 1 1] Flicker
      (`MaterialInstanceDynamic.SetScalarParameterValue` (`self.InnerMaterialFlicker`) "EmissiveBoost" (`KismetMathLibrary.RandomFloatInRange` 0.0 (`self.EmissiveBoost`)) :!label _label)
      (`KismetSystemLibrary.Delay` (`KismetMathLibrary.RandomFloatInRange` 0.0 (`self.RandomFlickerMaxOnTime`)))
      (goto _label))
    (:`NewEnumerator2`
      ;[1 1 1] Flash
      (`MaterialInstanceDynamic.SetScalarParameterValue` _innermaterial "EmissiveBoost" 0.0 :!label _label_2)
      (`KismetSystemLibrary.Delay` _flashmaxontime)
      (`MaterialInstanceDynamic.SetScalarParameterValue` _innermaterial "EmissiveBoost" (`self.EmissiveBoost`))
      (`KismetSystemLibrary.Delay` _flashmaxontime)
      (goto _label_2))
    (:`NewEnumerator3`
      ;[1 1 1] Off
      (`MaterialInstanceDynamic.SetScalarParameterValue` (`self.InnerMaterial`) "EmissiveBoost" 0.0))))

(fn `UserConstructionScript`
  (bind _chararray (`self.CharArray`))
  (bind _color (`self.Color`))
  (bind _innermaterial (`self.InnerMaterial`))
  (`|ExecutionSequence`
    (:`then_0`
      (bind _returnvalue (`KismetMaterialLibrary.CreateDynamicMaterialInstance` "/Game/RealNeonSignCreator/Materials/MI_NeonTube_Inner.MI_NeonTube_Inner"))
      (set `self.InnerMaterial` _returnvalue)
      (bind _returnvalue_2 (`KismetMaterialLibrary.CreateDynamicMaterialInstance` "/Game/RealNeonSignCreator/Materials/MI_NeonTube_Outer.MI_NeonTube_Outer"))
      (set `self.OuterMaterial` _returnvalue_2)
      (bind _returnvalue_3 (`KismetMaterialLibrary.CreateDynamicMaterialInstance` "/Game/RealNeonSignCreator/Materials/MI_BlackInsulated.MI_BlackInsulated"))
      (set `self.InsulatedMaterial` _returnvalue_3)
      (bind _returnvalue_4 (`KismetMaterialLibrary.CreateDynamicMaterialInstance` "/Game/RealNeonSignCreator/Materials/MI_NeonTube_Inner_Flicker.MI_NeonTube_Inner_Flicker"))
      (set `self.InnerMaterialFlicker` _returnvalue_4))
    (:`then_1`
      (`KismetArrayLibrary.Array_Clear` (`self.CharArray`))
      (for (_array_element _array_index) (`KismetStringLibrary.GetCharacterArrayFromString` (`self.Text`))
        (bind (_value _returnvalue_5) (`BlueprintMapLibrary.Map_Find` (`self.CharToMesh`) _array_element))
        (if _returnvalue_5
          (bind _returnvalue_6 (`AddComponent|NODE_AddStaticMeshComponent-4` :`RelativeTransform` (`KismetMathLibrary.MakeTransform` (`KismetMathLibrary.MakeVector` (* _array_index (`self.CharSpacing_X`)) (* _array_index (`self.CharSpacing_Y`))) (`KismetMathLibrary.MakeRotator` (`self.CharRotation_X`) (`self.CharRotation_Y`) (`self.CharRotation_Z`)) (`KismetMathLibrary.MakeVector` (`self.CharScale_X`) (`self.CharScale_Y`) 1.0))))
          (`KismetArrayLibrary.Array_Add` (`self.CharArray`) _returnvalue_6)
          (`SceneComponent.K2_AttachToComponent` _returnvalue_6 (`self.DefaultSceneRoot`) "None" "KeepRelative" "KeepRelative" "KeepRelative" true)
          (`StaticMeshComponent.SetStaticMesh` _returnvalue_6 _value)
          (`PrimitiveComponent.SetMaterial` _returnvalue_6 0 (`self.OuterMaterial`))
          (`PrimitiveComponent.SetMaterial` _returnvalue_6 1 _innermaterial)
          (`PrimitiveComponent.SetMaterial` _returnvalue_6 2 (`self.InsulatedMaterial`))
          (`MaterialInstanceDynamic.SetVectorParameterValue` _innermaterial "Color" _color)
          (`MaterialInstanceDynamic.SetVectorParameterValue` (`self.InnerMaterialFlicker`) "Color" _color)
          (`MaterialInstanceDynamic.SetScalarParameterValue` _innermaterial "EmissiveBoost" (`self.EmissiveBoost`))))
      (switch `/Game/RealNeonSignCreator/Blueprints/ENeonSignMode` (`self.NeonSignMode`)
        (:`NewEnumerator1`
          ;[1 1 1] Flicker
          (`PrimitiveComponent.SetMaterial` (`|GetArrayItem` _chararray (`KismetMathLibrary.RandomIntegerInRangeFromStream` 0 (- (`KismetArrayLibrary.Array_Length` _chararray) 1) (`self.RandomFlickerSeed`))) 1 (`self.InnerMaterialFlicker`)))))))
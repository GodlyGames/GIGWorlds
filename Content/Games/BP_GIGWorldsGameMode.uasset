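; Game mode for GIGWorlds that runs a tag game by periodically picking a random player to be "It".
; On login it records the controller and spawns an actor at a player start for it to possess.
; A looping timer clears and notifies every pawn, then tags one at random when at least two players are present.
; Cast targets and the spawned class are blank.
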(event `self.K2_PostLogin`
  (params (NewPlayer :type "PlayerController Object Reference"))
  (set `self.NewPlayer` NewPlayer)
  (`|ExecutionSequence`
    (:`then_0`
      (bind _returnvalue (`KismetArrayLibrary.Array_Add` (`self.PlayerControllers`) (`self.NewPlayer`)))
      (`KismetSystemLibrary.PrintString` (`KismetStringLibrary.Conv_IntToString` _returnvalue)))
    (:`then_3`
      (bind _returnvalue_2 (`|SpawnActorFromClass` null (`self.GetTransform` (`self.K2_FindPlayerStart` (`self.NewPlayer`) "1")) "AdjustIfPossibleButAlwaysSpawn" "OverrideRootScale" null null))
      (`Controller.Possess` (`self.NewPlayer`) _returnvalue_2))))

(event `self.ReceiveBeginPlay`
  ;[1 1 1] Starts Tag Game by randomly tagging a player every 180 seconds
  (`KismetSystemLibrary.K2_SetTimerDelegate` (delegate `Cycle Tag`) (`self.TagTimeSpan`) true))

(event `Cycle Tag`
  ;[1 1 1] Starts Tag Game by randomly tagging a player every 180 seconds
  (`|ExecutionSequence`
    (:`then_0`
      (bind _output_get (set `self.Player Array` (`GameStateBase.PlayerArray` (`GameplayStatics.GetGameState`))))
      (set `self.NumberOfPlayers` (`KismetArrayLibrary.Array_Length` _output_get)))
    (:`then_1`
      (for _array_element (`self.Player Array`)
        (bind _asbp_tag_person_character (cast `` (`PlayerState.PawnPrivate` _array_element)))
        (set `/Game/Games/BP_GIGWorldsGameMode.IsIt` false _asbp_tag_person_character)
        (message `/Game/Games/Tag/BPI_Tag.NotIt` _asbp_tag_person_character)))
    (:`then_2`
      (if (>= (`self.NumberOfPlayers`) 2)
        (bind _output_get_2 (set `self.Pawn Private` (`PlayerState.PawnPrivate` (`|GetArrayItem` (`self.Player Array`) (`KismetMathLibrary.RandomInteger` (`self.NumberOfPlayers`))))))
        (bind _asbp_tag_person_character_2 (cast `` _output_get_2))
        (set `/Game/Games/BP_GIGWorldsGameMode.IsIt` true _asbp_tag_person_character_2)
        (message `/Game/Games/Tag/BPI_Tag.YourIt` _asbp_tag_person_character_2)))))

(fn `OnRep_Pawn Private`
  (message `/Game/Games/Tag/BPI_Tag.YourIt` (`self.Pawn Private`)))

(fn `UserConstructionScript`)
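; Automatic two-panel sliding interior door for a sci-fi outpost, with a configurable locked state.
; Box overlap plays a timeline that slides both panels apart and reverses it on exit, unless LockTheDoor is set.
; Timelines drive the right panel's emissive light: red when locked or moving, cyan at start when unlocked and replayed after movement finishes.
; The construction script applies two configurable paint colors to both panels.
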(event `self.ReceiveBeginPlay`
  (bind _door_right (`self.Door Right`))
  (if (`self.Lock The Door `)
    ;[1 1 1] Door Blinking Light turns red if the door is locked  (Emissive Material)
    (bind (_direction _door_red_light) (`Timeline|Timeline_2`)
      (:`Update`
        (`MeshComponent.SetVectorParameterValueOnMaterials` _door_right "Glass/Emissive Color" (* (1.0 0.0 0.0) _door_red_light))
        (`MeshComponent.SetScalarParameterValueOnMaterials` _door_right "emission power" _door_red_light)))
    (else
      ;[1 1 1] Change Blinking light material color on Trigger overlap
      (bind (_direction_2 _door_red_light_2) (`Timeline|Timeline_1` :!label _label)
        (:`Update`
          (`MeshComponent.SetVectorParameterValueOnMaterials` (`self.Door Right`) "Glass/Emissive Color" (* (0.18 0.97 1.0) _door_red_light_2)))))))

(event `self.Box.OnComponentBeginOverlap`
  (params (OverlappedComponent :type "PrimitiveComponent Object Reference") (OtherActor :type "Actor Object Reference") (OtherComp :type "PrimitiveComponent Object Reference") (OtherBodyIndex :type Integer) (bFromSweep :type Boolean) (SweepResult :type "HitResult Structure (by ref)"))
  (bind _door_right (`self.Door Right`))
  ;[1 1 1] Opening/Closing door animtion on door trigger overlap
  (if (not (`self.Lock The Door `))
    (bind (_direction _left _right) (`Timeline|Timeline_0` :!label _label_2)
      (:`Update`
        (`SceneComponent.K2_SetRelativeLocation` (`self.Door Left`) (`KismetMathLibrary.MakeVector` _left -86.843094 1.484253) false false)
        (`SceneComponent.K2_SetRelativeLocation` _door_right (`KismetMathLibrary.MakeVector` _right -86.842926 1.484253) false false)
        ;[1 1 1] Change Blinking light material color on Trigger overlap
        (`MeshComponent.SetVectorParameterValueOnMaterials` _door_right "Glass/Emissive Color" (1.0 0.0 0.0)))
      (:`Finished`
        (goto _label)))))

(event `self.Box.OnComponentEndOverlap`
  (params (OverlappedComponent :type "PrimitiveComponent Object Reference") (OtherActor :type "Actor Object Reference") (OtherComp :type "PrimitiveComponent Object Reference") (OtherBodyIndex :type Integer))
  ;[1 1 1] Opening/Closing door animtion on door trigger overlap
  (if (not (`self.Lock The Door `))
    (goto _label_2 :!via `Reverse`)))

(fn `UserConstructionScript`
  (bind _door_right (`self.Door Right`))
  ;[1 1 1] Set Doors Color (Material)
  (`MeshComponent.SetVectorParameterValueOnMaterials` _door_right "Paint Color 2" (`KismetMathLibrary.Conv_LinearColorToVector` (`self.Door color 1`)))
  (`MeshComponent.SetVectorParameterValueOnMaterials` (`self.Door Left`) "Paint Color 2" (`KismetMathLibrary.Conv_LinearColorToVector` (`self.Door color 1`)))
  (`MeshComponent.SetVectorParameterValueOnMaterials` _door_right "Paint Color 3" (`KismetMathLibrary.Conv_LinearColorToVector` (`self.Door Color 2`)))
  (`MeshComponent.SetVectorParameterValueOnMaterials` (`self.Door Left`) "Paint Color 3" (`KismetMathLibrary.Conv_LinearColorToVector` (`self.Door Color 2`))))
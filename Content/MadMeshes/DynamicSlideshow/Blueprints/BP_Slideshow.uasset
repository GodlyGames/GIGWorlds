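; Slideshow actor that cycles textures on a display mesh through a dynamic material instance, using static images, downloaded URLs or Twitch Live channel images.
; Once powered on, a timer drives image selection by mode; online and Twitch modes set a static fallback texture before downloading, with a 404 texture for failed downloads.
; Static images and URLs move to "used" arrays as shown, in order or randomized, and refill when exhausted.
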(event `self.ReceiveBeginPlay`
  ;[0 1 0] Turn on if Power On is true
  (if (`self.PowerOn`)
    (`self.TurnOn`)))

(event `TurnOn`
  ;[0 0 1] Power On and start timed event for changing images
  (bind _returnvalue (`KismetSystemLibrary.K2_SetTimer` null "EventLoadNextImage" (`self.CycleImageInSeconds`) (`self.Looping`) (`self.StartupDelay`)))
  (set `self.CycleImageTimer` _returnvalue)
  (set `self.PowerOn` true)
  (`KismetSystemLibrary.Delay` (`self.StartupDelay`))
  (`self.EventLoadNextImage`))

(event `LoadFallbackImage`
  ;[0.5 0.5 0] Determine which mode the slideshow is in  Static, Online or from TwitchLive
  (set `self.ImageParameterName` "FallbackImage")
  (bind (_ready _nextimageindex) (`self.SelectNextImage` :!label _label))
  (if _ready
    (set `self.SelectedImageIndex` _nextimageindex)
    (`|ExecutionSequence`
      (:`then_0`
        (set `self.SelectedImage` (`|GetArrayItem` (`self.StaticImages`) (`self.SelectedImageIndex`))))
      (:`then_4`
        (`KismetArrayLibrary.Array_Remove` (`self.StaticImages`) (`self.SelectedImageIndex`))
        (`KismetArrayLibrary.Array_Add` (`self.StaticImages_Used`) (`self.SelectedImage`)))
      (:`then_9`
        (`MaterialInstanceDynamic.SetTextureParameterValue` (`self.DynamicMaterialInstance`) (`self.ImageParameterName`) (`self.SelectedImage`))
        ;;[1 1 1] In case it was a fallback image
        (set `self.ImageParameterName` "NewImage")))
    (else
      (`KismetSystemLibrary.PrintString` "No Images In Array" true true (struct :`R` 1.0 :`A` 1.0) 10.0))))

(event `EventLoadNextImage`
  ;[0.5 0.5 0] Determine which mode the slideshow is in  Static, Online or from TwitchLive
  (switch `/Game/MadMeshes/DynamicSlideshow/Blueprints/E_Slideshow` (`self.SlideshowType`)
    (:`NewEnumerator0`
      (goto _label))
    (:`NewEnumerator1`
      (`self.LoadFallbackImage`)
      (bind (_ready _returnvalue) (`self.SelectNextUrl`))
      (if _ready
        (set `self.SelectedUrlIndex` _returnvalue)
        (`|ExecutionSequence`
          (:`then_0`
            (set `self.OnlineImageUrl` (`|GetArrayItem` (`self.OnlineImageUrls`) (`self.SelectedUrlIndex`))))
          (:`then_4`
            (`KismetArrayLibrary.Array_Remove` (`self.OnlineImageUrls`) (`self.SelectedUrlIndex`))
            (`KismetArrayLibrary.Array_Add` (`self.OnlineImageUrls_Used`) (`self.OnlineImageUrl`)))
          (:`then_9`
            (bind _returnvalue_2 (`self.FormatUrl` "{input}" (`self.OnlineImageUrl`))
              (:`then`
                (bind _texture (`AsyncTaskDownloadImage.DownloadImage` _returnvalue_2)
                  (:`OnSuccess`
                    (set `self.DownloadedImage` _texture))
                  (:`OnFail`
                    (set `self.DownloadedImage` "/Game/MadMeshes/DynamicSlideshow/Textures/T_404_preview.T_404_preview"))))))
          (:`then_14`
            (`MaterialInstanceDynamic.SetTextureParameterValue` (`self.DynamicMaterialInstance`) (`self.ImageParameterName`) (`self.DownloadedImage`) :!label _label_2)))
        (else
          (`KismetSystemLibrary.PrintString` "No URLs In Array" true true (struct :`R` 1.0 :`A` 1.0) 10.0)
          (goto _label_2))))
    (:`NewEnumerator2`
      (`self.LoadFallbackImage`)
      (bind _returnvalue_3 (`self.FormatUrl` (`self.TwitchLiveURL`) (`self.TwitchChannel`))
        (:`then`
          (bind _texture_2 (`AsyncTaskDownloadImage.DownloadImage` _returnvalue_3)
            (:`OnSuccess`
              (set `self.DownloadedImage` _texture_2)
              (`|ExecutionSequence`
                (:`then_0`
                  (bind _returnvalue_4 (`KismetArrayLibrary.Array_Add` (`self.TwitchImage_Used`) (`self.DownloadedImage`)))
                  (if (> _returnvalue_4 100)
                    (`KismetArrayLibrary.Array_Remove` (`self.TwitchImage_Used`))))
                (:`then_5`
                  (`MaterialInstanceDynamic.SetTextureParameterValue` (`self.DynamicMaterialInstance`) (`self.ImageParameterName`) (`self.DownloadedImage`)))))
            (:`OnFail`
              (`KismetSystemLibrary.PrintString` "ERROR:  Download Image Failed" true true (struct :`R` 1.0 :`A` 1.0) 10.0)
              (`MaterialInstanceDynamic.SetTextureParameterValue` (`self.DynamicMaterialInstance`) (`self.ImageParameterName`) "/Game/MadMeshes/DynamicSlideshow/Textures/T_404_preview.T_404_preview" :!label _label_3))))
        (:`Empty`
          (`KismetSystemLibrary.PrintString` "ERROR:  Empty Twitch Name" true true (struct :`R` 1.0 :`A` 1.0) 10.0)
          (goto _label_3))))))

(fn `SelectNextImage`
  (returns (Ready :type Boolean) (NextImageIndex :type Integer))
  ;[1 0 1] Checks to see if all the images have been used, and if so reloads the array.  Returns Ready = Fales - If both arrays are empty.
  (if (`KismetArrayLibrary.Array_IsValidIndex` (`self.StaticImages`))
    _
    (elif (`KismetArrayLibrary.Array_IsValidIndex` (`self.StaticImages_Used`))
      (`KismetArrayLibrary.Array_Append` (`self.StaticImages`) (`self.StaticImages_Used`))
      (`KismetArrayLibrary.Array_Clear` (`self.StaticImages_Used`))
      (else
        ;;[1 0 0] No Images In Arrays
        (return false 0))))
  (if (`self.Randomize`)
    (return true (`KismetMathLibrary.RandomIntegerInRange` 0 (`KismetArrayLibrary.Array_LastIndex` (`self.StaticImages`))))
    (else
      (return true 0))))

(fn `SelectNextUrl`
  (returns (Ready :type Boolean) (ReturnValue :type Integer))
  ;[1 0 1] Checks to see if all the urls have been used, and if so reloads the array.  Returns Ready = Fales - If both arrays are empty.
  (if (`KismetArrayLibrary.Array_IsValidIndex` (`self.OnlineImageUrls`))
    _
    (elif (`KismetArrayLibrary.Array_IsValidIndex` (`self.OnlineImageUrls_Used`))
      (`KismetArrayLibrary.Array_Append` (`self.OnlineImageUrls`) (`self.OnlineImageUrls_Used`))
      (`KismetArrayLibrary.Array_Clear` (`self.OnlineImageUrls_Used`))
      (else
        ;;[1 0 0] No Images In Arrays
        (return false 0))))
  (if (`self.Randomize`)
    (return true (`KismetMathLibrary.RandomIntegerInRange` 0 (`KismetArrayLibrary.Array_LastIndex` (`self.OnlineImageUrls`))))
    (else
      (return true 0))))

(fn `UserConstructionScript`
  (locals (NewLocalVar_0 :type "MaterialInstanceDynamic Object Reference"))
  ;[0 1 0] Setup material Instance on construction.
  (bind _returnvalue (`PrimitiveComponent.CreateDynamicMaterialInstance` (`self.DisplayImage`) (`self.Material Element Index`) "/Game/MadMeshes/DynamicSlideshow/Materials/MI_DisplayImage.MI_DisplayImage" "Screen"))
  (bind _output_get (set `self.DynamicMaterialInstance` _returnvalue))
  (`MaterialInstanceDynamic.SetTextureParameterValue` _output_get "NewImage" (`self.InitialDisplayImage`)))
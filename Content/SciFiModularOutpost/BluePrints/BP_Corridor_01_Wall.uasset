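; Modular sci-fi corridor wall that assembles its look from separate lower, middle and top variation selectors.
; The Construction Script handles each band independently, swapping panel meshes from per-band arrays indexed by the selected variation.
; Lower variations also destroy unneeded pipe and panel components, middle ones can toggle a lid's visibility, and top ones can change either or both panels.
; The event graph has no runtime logic.
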(fn `UserConstructionScript`
  (bind _select_middle_part_variation (`self.Select Middle Part Variation`))
  (bind _sm_gate_interior_panel_107_staticmeshcomponent0 (`self.SM_Gate_Interior_Panel_107_StaticMeshComponent0`))
  (bind _select_lower_part_variation (`self.Select Lower Part Variation`))
  (bind _select_higher_part_variation (`self.Select Higher Part Variation`))
  (bind _output (`|GetArrayItem` (`self.Static mesh Top`) (`KismetMathLibrary.Conv_ByteToInt` _select_higher_part_variation)))
  (`|ExecutionSequence`
    (:`then_0`
      ;[1 1 1] Lower Part
      (switch `/Game/SciFiModularOutpost/BluePrints/Enumerations/E_Interior_Wall_01_Variation_Lower` _select_lower_part_variation
        (:`NewEnumerator0`
          (`|ExecutionSequence`
            (:`then_0`
              (`ActorComponent.K2_DestroyComponent` (`self.SM_TubedPipe_010`) :!label _label)
              (`ActorComponent.K2_DestroyComponent` (`self.SM_TubedPipe_05`))
              (`ActorComponent.K2_DestroyComponent` (`self.SM_TubedPipe_08`))
              (`ActorComponent.K2_DestroyComponent` (`self.SM_TubedPipe_09`))
              (`ActorComponent.K2_DestroyComponent` (`self.SM_TubedPipe_04`)))
            (:`then_1`
              (`ActorComponent.K2_DestroyComponent` (`self.SM_pipe_Large_2m4`) :!label _label_2)
              (`ActorComponent.K2_DestroyComponent` (`self.SM_pipe_Large_2m1`))
              (`ActorComponent.K2_DestroyComponent` (`self.SM_pipe_Large_2m3`))
              (`ActorComponent.K2_DestroyComponent` (`self.SM_pipe_Large_2m2`))
              (`ActorComponent.K2_DestroyComponent` (`self.SM_pipe_Large_2m`)))))
        (:`NewEnumerator1`
          (`|ExecutionSequence`
            (:`then_0`
              (goto _label_2))
            (:`then_1`
              (`StaticMeshComponent.SetStaticMesh` (`self.SM_Gate_Interior_Panel_104_StaticMeshComponent0`) (`|GetArrayItem` (`self.Static mesh Lower`) (`KismetMathLibrary.Conv_ByteToInt` _select_lower_part_variation)) :!label _label_3)
              (`ActorComponent.K2_DestroyComponent` (`self.SM_Gate_Interior_Panel_103_StaticMeshComponent0`)))))
        (:`NewEnumerator3`
          (`|ExecutionSequence`
            (:`then_0`
              (goto _label))
            (:`then_1`
              (goto _label_3))))))
    (:`then_1`
      ;[1 1 1] Middle Part
      (switch `/Game/SciFiModularOutpost/BluePrints/Enumerations/E_Interior_Wall_01_Variation_Middle` _select_middle_part_variation
        (:`NewEnumerator0`
          (`SceneComponent.ToggleVisibility` (`self.SM_Gate_Interior_Panel_10_lid`) false))
        (:`NewEnumerator1`
          (`StaticMeshComponent.SetStaticMesh` (`self.SM_Gate_Interior_Panel_105_StaticMeshComponent0`) (`|GetArrayItem` (`self.Static mesh Middle`) (`KismetMathLibrary.Conv_ByteToInt` _select_middle_part_variation))))
        (:`NewEnumerator3`
          (`StaticMeshComponent.SetStaticMesh` (`self.SM_Gate_Interior_Panel_105_StaticMeshComponent0`) (`|GetArrayItem` (`self.Static mesh Middle`) (`KismetMathLibrary.Conv_ByteToInt` (`self.Select Middle Part Variation`))))
          (`SceneComponent.ToggleVisibility` (`self.SM_Gate_Interior_Panel_10_lid`) false))))
    (:`then_2`
      ;[1 1 1] Top Part
      (switch `/Game/SciFiModularOutpost/BluePrints/Enumerations/E_Interior_Wall_01_Variation_Top` _select_higher_part_variation
        (:`NewEnumerator1`
          (`StaticMeshComponent.SetStaticMesh` _sm_gate_interior_panel_107_staticmeshcomponent0 _output)
          (`StaticMeshComponent.SetStaticMesh` (`self.SM_Gate_Interior_Panel_106_StaticMeshComponent0`) _output :!label _label_4))
        (:`NewEnumerator3`
          (goto _label_4))
        (:`NewEnumerator4`
          (`StaticMeshComponent.SetStaticMesh` _sm_gate_interior_panel_107_staticmeshcomponent0 _output))))))
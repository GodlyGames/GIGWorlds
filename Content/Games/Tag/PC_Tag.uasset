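; PC_Tag is the player controller for a Tag game, holding whether its player is currently "it".
; On possession it stores the pawn as a BP_TagCharacter.
; The YourIt and NotIt events set Tagged and forward it to that character's Tag call.
; Tagged has an OnRep, but its body is empty, with the pawn update and debug prints left disconnected.
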(event `self.ReceiveBeginPlay`)

(event `self.ReceivePossess`
  (params (PossessedPawn :type "Pawn Object Reference"))
  ;[1 0.5 0] On Possession
  (bind _asbp_tag_character (cast `/Game/Games/Tag/BP_TagCharacter` PossessedPawn))
  (set `self.PossessedPawn` _asbp_tag_character))

(event `self.NotIt`
  ;[1 0.5 0] Not It Event
  (bind _output_get (set `self.Tagged` false))
  (`/Game/Games/Tag/BP_TagCharacter.Tag` (`self.PossessedPawn`) _output_get))

(event `self.YourIt`
  ;[1 0.5 0] Tagged Event
  (bind _output_get (set `self.Tagged` true))
  (`/Game/Games/Tag/BP_TagCharacter.Tag` (`self.PossessedPawn`) _output_get))

(fn `OnRep_Tagged`)

(fn `UserConstructionScript`)
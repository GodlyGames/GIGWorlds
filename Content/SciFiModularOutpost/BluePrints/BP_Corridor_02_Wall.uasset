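; BP_Corridor_02_Wall is a modular sci-fi corridor wall piece that configures its look in the construction script, with no active event logic.
; The middle-part selection destroys the panel components its variation does not use, with Variation 2 also swapping in a mesh from MeshMiddle.
; Two panels receive a connection material, whose texture offset and UV scale parameters are then adjusted by the trim selection.
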(fn `UserConstructionScript`
  (bind _sm_gate_interior_panel_136_sm_gate_interior_panel_99_staticmeshcomponent0 (`self.SM_Gate_Interior_Panel_136_SM_Gate_Interior_Panel_99_StaticMeshComponent0`))
  (bind _select_middle_part_variation (`self.Select Middle Part Variation`))
  (`PrimitiveComponent.SetMaterial` (`self.SM_Gate_Interior_Panel_136_SM_Gate_Interior_Panel_99_StaticMeshComponent0`) 1 "/Game/SciFiModularOutpost/Materials/MaterialInstances/MI_Connection_06.MI_Connection_06")
  (`PrimitiveComponent.SetMaterial` (`self.SM_Gate_Interior_Panel_136_SM_Gate_Interior_Panel_61_StaticMeshComponent0`) 1 "/Game/SciFiModularOutpost/Materials/MaterialInstances/MI_Connection_06.MI_Connection_06")
  (`|ExecutionSequence`
    (:`then_0`
      ;[1 1 1] Select Middle Part Var
      (switch `/Game/SciFiModularOutpost/BluePrints/Enumerations/E_Interior_Wall_01_Variation_Middle` _select_middle_part_variation
        (:`NewEnumerator0`
          (`ActorComponent.K2_DestroyComponent` (`self.SM_Gate_Interior_Panel_136_SM_Gate_Interior_Panel_106_StaticMeshComponent1`) :!label _label)
          (`ActorComponent.K2_DestroyComponent` (`self.SM_Gate_Interior_Panel_136_SM_Gate_Interior_Panel_106_StaticMeshComponent2`)))
        (:`NewEnumerator1`
          (`StaticMeshComponent.SetStaticMesh` (`self.SM_Gate_Interior_Panel_136_SM_Gate_Interior_Panel_63_StaticMeshComponent1`) (`|GetArrayItem` (`self.Mesh middle`) (`KismetMathLibrary.Conv_ByteToInt` _select_middle_part_variation)))
          (goto _label))
        (:`NewEnumerator3`
          (`ActorComponent.K2_DestroyComponent` (`self.SM_Gate_Interior_Panel_136_SM_Gate_Interior_Panel_106_StaticMeshComponent0`))
          (`ActorComponent.K2_DestroyComponent` (`self.SM_Gate_Interior_Panel_136_SM_Gate_Interior_Panel_117_StaticMeshComponent0`))
          (`ActorComponent.K2_DestroyComponent` (`self.SM_Gate_Interior_Panel_136_SM_Gate_Interior_Panel_62_StaticMeshComponent0`))
          (`ActorComponent.K2_DestroyComponent` (`self.SM_Gate_Interior_Panel_136_SM_Gate_Interior_Panel_105_StaticMeshComponent0`)))))
    (:`then_1`
      ;[1 1 1] Set Material Variation
      (switch `/Game/SciFiModularOutpost/BluePrints/Enumerations/E_Interior_Wall_01_Variation_Middle` (`self.Select Trim Variation`)
        (:`NewEnumerator1`
          (`MeshComponent.SetScalarParameterValueOnMaterials` _sm_gate_interior_panel_136_sm_gate_interior_panel_99_staticmeshcomponent0 "Texture Offset Y" 1.85)
          (`MeshComponent.SetScalarParameterValueOnMaterials` (`self.SM_Gate_Interior_Panel_136_SM_Gate_Interior_Panel_61_StaticMeshComponent0`) "Texture Offset Y" 1.85)
          (`MeshComponent.SetScalarParameterValueOnMaterials` _sm_gate_interior_panel_136_sm_gate_interior_panel_99_staticmeshcomponent0 "Texture UV Size" 0.550137)
          (`MeshComponent.SetScalarParameterValueOnMaterials` (`self.SM_Gate_Interior_Panel_136_SM_Gate_Interior_Panel_61_StaticMeshComponent0`) "Texture UV Size" 0.550137))
        (:`NewEnumerator3`
          (`MeshComponent.SetScalarParameterValueOnMaterials` _sm_gate_interior_panel_136_sm_gate_interior_panel_99_staticmeshcomponent0 "Texture Offset Y" 0.0)
          (`MeshComponent.SetScalarParameterValueOnMaterials` (`self.SM_Gate_Interior_Panel_136_SM_Gate_Interior_Panel_61_StaticMeshComponent0`) "Texture Offset Y" 0.0))))))
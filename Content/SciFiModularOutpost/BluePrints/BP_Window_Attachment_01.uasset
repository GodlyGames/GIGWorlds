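; BP_Window_Attachment_01 is a modular sci-fi outpost window attachment prop with two selectable mesh variations and an adjustable paint color.
; The Construction Script switches on SelectAttachmentType and destroys the static mesh component of the unused variation.
; It then assigns that variation's material and pushes SetPaintColor into a paint color vector parameter, whose name differs per variation.
; The event graph holds only disabled placeholder events, so there is no runtime logic.
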(fn `UserConstructionScript`
  (bind _wall_01_attachment_a16_staticmeshcomponent0 (`self.Wall_01_attachment_a16_StaticMeshComponent0`))
  (bind _set_paint_color (`self.Set Paint Color`))
  ;[1 1 1] Select Wall Attachment Variation Type
  (switch `/Game/SciFiModularOutpost/BluePrints/Enumerations/E_WindowAttachment_Choose` (`self.Select Attachment Type`)
    (:`NewEnumerator0`
      ;[1 1 1] Variaiton 1
      (`ActorComponent.K2_DestroyComponent` (`self.SM_WallAttachment_02`))
      ;;[1 1 1] Set Material and Color
      (`PrimitiveComponent.SetMaterial` _wall_01_attachment_a16_staticmeshcomponent0 1 "/Game/SciFiModularOutpost/Materials/MaterialInstances/MI_Attachment_Trim1.MI_Attachment_Trim1")
      (`MeshComponent.SetVectorParameterValueOnMaterials` _wall_01_attachment_a16_staticmeshcomponent0 "Paint Color" (`KismetMathLibrary.Conv_LinearColorToVector` _set_paint_color)))
    (:`NewEnumerator1`
      ;[1 1 1] Variaiton 2
      (`ActorComponent.K2_DestroyComponent` _wall_01_attachment_a16_staticmeshcomponent0)
      ;;[1 1 1] Set Material and Color
      (`PrimitiveComponent.SetMaterial` _wall_01_attachment_a16_staticmeshcomponent0 0 "/Game/SciFiModularOutpost/Materials/MaterialInstances/MI_Attach.MI_Attach")
      (`PrimitiveComponent.SetMaterial` (`self.SM_WallAttachment_02`) 0 "/Game/SciFiModularOutpost/Materials/MaterialInstances/MI_Attach.MI_Attach")
      (`MeshComponent.SetVectorParameterValueOnMaterials` _wall_01_attachment_a16_staticmeshcomponent0 "Paint Color 2" (`KismetMathLibrary.Conv_LinearColorToVector` _set_paint_color))
      (`MeshComponent.SetVectorParameterValueOnMaterials` (`self.SM_WallAttachment_02`) "Paint Color 2" (`KismetMathLibrary.Conv_LinearColorToVector` _set_paint_color)))))
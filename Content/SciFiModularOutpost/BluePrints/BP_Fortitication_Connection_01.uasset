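; Modular fortification connection piece for the sci-fi outpost, configured entirely in the Construction Script as a one- or two-sided wall section.
; One-sided mode destroys the second side's meshes and light.
; A selector swaps between two pillar meshes or a flat wall, which hides the pillars, lights and associated wall pieces.
; For pillars, shared intensity and color settings drive both the point lights and the materials' emissive parameters.
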(fn `UserConstructionScript`
  (bind _pointlight1 (`self.PointLight1`))
  (bind _light_color (`self.Light Color`))
  (bind _pointlight1_2 (`self.PointLight1`))
  (bind _light_intensity (`self.Light Intensity`))
  (bind _light_color_2 (`self.Light Color`))
  (bind _light_intensity_2 (`self.Light Intensity`))
  (bind _plane1 (`self.Plane1`))
  (bind _plane2 (`self.Plane2`))
  (bind _plane1_2 (`self.Plane1`))
  (bind _plane1_3 (`self.Plane1`))
  (bind _plane1_4 (`self.Plane1`))
  ;[1 1 1] Choose whether the wall is one sided or 2sided
  (switch `/Game/SciFiModularOutpost/BluePrints/Enumerations/E_Fortification_Pillar_Sides` (`self.pillar Sides`)
    (:`NewEnumerator1`
      ;[1 1 1] Select Pillar Type (2 Sided)
      (switch `/Game/SciFiModularOutpost/BluePrints/Enumerations/E_Fortification_Pillar_Choose` (`self.Select Pillar Type`)
        (:`NewEnumerator1`
          (`StaticMeshComponent.SetStaticMesh` _plane1 "/Game/SciFiModularOutpost/StaticMeshes/SM_Fortification_Pillar_01.SM_Fortification_Pillar_01")
          (`StaticMeshComponent.SetStaticMesh` _plane2 "/Game/SciFiModularOutpost/StaticMeshes/SM_Fortification_Pillar_01.SM_Fortification_Pillar_01")
          ;[1 1 1] Local Lighting 2 sided
          (`LightComponent.SetIntensity` _pointlight1_2 _light_intensity :!label _label)
          (`LightComponent.SetIntensity` (`self.PointLight2`) _light_intensity)
          (`LightComponent.SetLightColor` _pointlight1_2 _light_color_2 true)
          (`LightComponent.SetLightColor` (`self.PointLight2`) _light_color_2 true)
          (`MeshComponent.SetScalarParameterValueOnMaterials` _plane1_2 "Emission Power" (`KismetMathLibrary.SafeDivide` _light_intensity 1000.0))
          (`MeshComponent.SetScalarParameterValueOnMaterials` (`self.Plane2`) "Emission Power" (`KismetMathLibrary.SafeDivide` _light_intensity 1000.0))
          (`MeshComponent.SetVectorParameterValueOnMaterials` _plane1_2 "Glass/Emissive Color" (`KismetMathLibrary.Conv_LinearColorToVector` _light_color_2))
          (`MeshComponent.SetVectorParameterValueOnMaterials` (`self.Plane2`) "Glass/Emissive Color" (`KismetMathLibrary.Conv_LinearColorToVector` _light_color_2)))
        (:`NewEnumerator2`
          (`StaticMeshComponent.SetStaticMesh` _plane1 "/Game/SciFiModularOutpost/StaticMeshes/SM_Fortification_Pillar_02.SM_Fortification_Pillar_02")
          (`StaticMeshComponent.SetStaticMesh` _plane2 "/Game/SciFiModularOutpost/StaticMeshes/SM_Fortification_Pillar_02.SM_Fortification_Pillar_02")
          (goto _label))
        (:`NewEnumerator3`
          (`SceneComponent.ToggleVisibility` _plane1 false)
          (`SceneComponent.ToggleVisibility` _plane2 false)
          (`SceneComponent.ToggleVisibility` (`self.SM_wall_01_2m_a9`) false)
          (`SceneComponent.ToggleVisibility` (`self.SM_wall_01_2m_a10`) false)
          (`SceneComponent.ToggleVisibility` (`self.SM_wall_01_2m_a11`) false)
          (`SceneComponent.ToggleVisibility` (`self.PointLight2`) false)
          (`SceneComponent.ToggleVisibility` (`self.PointLight1`) false)
          (`SceneComponent.ToggleVisibility` (`self.SM_wall_01_2m_a2`) false)
          (`SceneComponent.ToggleVisibility` (`self.SM_wall_01_2m_a1`) false)
          (`SceneComponent.ToggleVisibility` (`self.SM_wall_01_2m_a`) false)
          (`SceneComponent.ToggleVisibility` (`self.SM_wall_01_2m_a3`) false))))
    (:`NewEnumerator2`
      ;[1 1 1] Destroy Elements if the asset is chosen to be one sided
      (`ActorComponent.K2_DestroyComponent` (`self.Plane2`))
      (`ActorComponent.K2_DestroyComponent` (`self.PointLight2`))
      (`ActorComponent.K2_DestroyComponent` (`self.SM_wall_01_2m_a8`))
      (`ActorComponent.K2_DestroyComponent` (`self.SM_wall_01_2m_a11`))
      (`ActorComponent.K2_DestroyComponent` (`self.SM_wall_01_2m_a10`))
      (`ActorComponent.K2_DestroyComponent` (`self.SM_wall_01_2m_a9`))
      (`ActorComponent.K2_DestroyComponent` (`self.SM_Gate_Interior_Panel_53_StaticMeshComponent0`))
      ;[1 1 1] Select Pillar Type (1 Sided)
      (switch `/Game/SciFiModularOutpost/BluePrints/Enumerations/E_Fortification_Pillar_Choose` (`self.Select Pillar Type`)
        (:`NewEnumerator1`
          (`StaticMeshComponent.SetStaticMesh` _plane1_3 "/Game/SciFiModularOutpost/StaticMeshes/SM_Fortification_Pillar_01.SM_Fortification_Pillar_01")
          ;[1 1 1] Local Lighting 1 Sided
          (`LightComponent.SetIntensity` _pointlight1 _light_intensity_2 :!label _label_2)
          (`LightComponent.SetLightColor` _pointlight1 _light_color true)
          (`MeshComponent.SetScalarParameterValueOnMaterials` _plane1_4 "Emission Power" (`KismetMathLibrary.SafeDivide` _light_intensity_2 1000.0))
          (`MeshComponent.SetVectorParameterValueOnMaterials` _plane1_4 "Glass/Emissive Color" (`KismetMathLibrary.Conv_LinearColorToVector` _light_color)))
        (:`NewEnumerator2`
          (`StaticMeshComponent.SetStaticMesh` _plane1_3 "/Game/SciFiModularOutpost/StaticMeshes/SM_Fortification_Pillar_02.SM_Fortification_Pillar_02")
          (goto _label_2))
        (:`NewEnumerator3`
          (`SceneComponent.ToggleVisibility` _plane1_3 false)
          (`SceneComponent.ToggleVisibility` (`self.PointLight1`) false)
          (`SceneComponent.ToggleVisibility` (`self.SM_wall_01_2m_a2`) false)
          (`SceneComponent.ToggleVisibility` (`self.SM_wall_01_2m_a1`) false)
          (`SceneComponent.ToggleVisibility` (`self.SM_wall_01_2m_a`) false)
          (`SceneComponent.ToggleVisibility` (`self.SM_wall_01_2m_a3`) false))))))
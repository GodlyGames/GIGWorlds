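; Modular sci-fi outpost fortification wall Blueprint that can be shown as one-sided or two-sided.
; The Construction Script switches on the Sides setting, and for a one-sided wall the SwitchSide bool picks which face to remove.
; The hidden face is removed by calling DestroyComponent on its hard-wired list of static mesh panel components.
; The Event Graph holds only disabled placeholder events, so there is no runtime logic.
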(fn `UserConstructionScript`
  ;[1 1 1] Choose whether the wall is one sided or 2sided
  (switch `/Game/SciFiModularOutpost/BluePrints/Enumerations/E_Fotification_2Side` (`self.Sides`)
    (:`NewEnumerator5`
      ;[1 1 1] Swap visible wall side
      (if (`self.Switch Side`)
        ;[1 1 1] Destroy the back side if selected as invisble
        (`ActorComponent.K2_DestroyComponent` (`self.SM_Gate_Interior_Panel_1124_StaticMeshComponent0`))
        (`ActorComponent.K2_DestroyComponent` (`self.SM_Gate_Interior_Panel_1146_StaticMeshComponent0`))
        (`ActorComponent.K2_DestroyComponent` (`self.SM_Gate_Interior_Panel_1143_StaticMeshComponent0`))
        (`ActorComponent.K2_DestroyComponent` (`self.SM_Gate_Interior_Panel_1140_StaticMeshComponent0`))
        (`ActorComponent.K2_DestroyComponent` (`self.SM_Gate_Interior_Panel_1103_StaticMeshComponent0`))
        (`ActorComponent.K2_DestroyComponent` (`self.SM_Gate_Interior_Panel_1139_StaticMeshComponent0`))
        (`ActorComponent.K2_DestroyComponent` (`self.SM_Gate_Interior_Panel_1131_StaticMeshComponent0`))
        (`ActorComponent.K2_DestroyComponent` (`self.SM_Gate_Interior_Panel_1132_StaticMeshComponent0`))
        (`ActorComponent.K2_DestroyComponent` (`self.SM_Gate_Interior_Panel_1133_StaticMeshComponent0`))
        (`ActorComponent.K2_DestroyComponent` (`self.SM_Gate_Interior_Panel_1134_StaticMeshComponent0`))
        (`ActorComponent.K2_DestroyComponent` (`self.SM_Gate_Interior_Panel_1135_StaticMeshComponent0`))
        (`ActorComponent.K2_DestroyComponent` (`self.SM_Gate_Interior_Panel_1136_StaticMeshComponent0`))
        (`ActorComponent.K2_DestroyComponent` (`self.SM_Gate_Interior_Panel_1137_StaticMeshComponent0`))
        (`ActorComponent.K2_DestroyComponent` (`self.SM_Gate_Interior_Panel_1138_StaticMeshComponent0`))
        (`ActorComponent.K2_DestroyComponent` (`self.SM_Gate_Interior_Panel_1117_StaticMeshComponent0`))
        (`ActorComponent.K2_DestroyComponent` (`self.SM_Gate_Interior_Panel_1118_StaticMeshComponent0`))
        (`ActorComponent.K2_DestroyComponent` (`self.SM_Gate_Interior_Panel_1119_StaticMeshComponent0`))
        (`ActorComponent.K2_DestroyComponent` (`self.SM_Gate_Interior_Panel_1120_StaticMeshComponent0`))
        (`ActorComponent.K2_DestroyComponent` (`self.SM_Gate_Interior_Panel_1121_StaticMeshComponent0`))
        (`ActorComponent.K2_DestroyComponent` (`self.SM_Gate_Interior_Panel_1122_StaticMeshComponent0`))
        (`ActorComponent.K2_DestroyComponent` (`self.SM_Gate_Interior_Panel_1123_StaticMeshComponent0`))
        (`ActorComponent.K2_DestroyComponent` (`self.SM_Gate_Interior_Panel_1149_StaticMeshComponent0`))
        (`ActorComponent.K2_DestroyComponent` (`self.SM_Gate_Interior_Panel_1106_StaticMeshComponent0`))
        (`ActorComponent.K2_DestroyComponent` (`self.SM_Gate_Interior_Panel_1107_StaticMeshComponent0`))
        (`ActorComponent.K2_DestroyComponent` (`self.SM_Gate_Interior_Panel_1109_StaticMeshComponent0`))
        (`ActorComponent.K2_DestroyComponent` (`self.SM_Gate_Interior_Panel_1110_StaticMeshComponent0`))
        (`ActorComponent.K2_DestroyComponent` (`self.SM_Gate_Interior_Panel_1111_StaticMeshComponent0`))
        (`ActorComponent.K2_DestroyComponent` (`self.SM_Gate_Interior_Panel_1112_StaticMeshComponent0`))
        (`ActorComponent.K2_DestroyComponent` (`self.SM_Gate_Interior_Panel_1113_StaticMeshComponent0`))
        (`ActorComponent.K2_DestroyComponent` (`self.SM_Gate_Interior_Panel_1114_StaticMeshComponent0`))
        (`ActorComponent.K2_DestroyComponent` (`self.SM_Gate_Interior_Panel_1115_StaticMeshComponent0`))
        (`ActorComponent.K2_DestroyComponent` (`self.SM_Gate_Interior_Panel_1116_StaticMeshComponent0`))
        (`ActorComponent.K2_DestroyComponent` (`self.SM_Gate_Interior_Panel_1105_StaticMeshComponent0`))
        (`ActorComponent.K2_DestroyComponent` (`self.SM_Gate_Interior_Panel_1104_StaticMeshComponent0`))
        (`ActorComponent.K2_DestroyComponent` (`self.SM_Gate_Interior_Panel_1125_StaticMeshComponent0`))
        (`ActorComponent.K2_DestroyComponent` (`self.SM_Gate_Interior_Panel_1126_StaticMeshComponent0`))
        (`ActorComponent.K2_DestroyComponent` (`self.SM_Gate_Interior_Panel_1127_StaticMeshComponent0`))
        (`ActorComponent.K2_DestroyComponent` (`self.SM_Gate_Interior_Panel_1128_StaticMeshComponent0`))
        (`ActorComponent.K2_DestroyComponent` (`self.SM_Gate_Interior_Panel_1102_StaticMeshComponent0`))
        (`ActorComponent.K2_DestroyComponent` (`self.SM_Gate_Interior_Panel_1101_StaticMeshComponent0`))
        (`ActorComponent.K2_DestroyComponent` (`self.SM_Gate_Interior_Panel_1100_StaticMeshComponent0`))
        (`ActorComponent.K2_DestroyComponent` (`self.SM_Gate_Interior_Panel_1108_StaticMeshComponent4`))
        (`ActorComponent.K2_DestroyComponent` (`self.SM_Gate_Interior_Panel_1100_StaticMeshComponent1`))
        (`ActorComponent.K2_DestroyComponent` (`self.SM_Gate_Interior_Panel_1108_StaticMeshComponent6`))
        (else
          ;[1 1 1] Destroy the front side if selected as invisble
          (`ActorComponent.K2_DestroyComponent` (`self.SM_Gate_Interior_Panel_1157_StaticMeshComponent0`))
          (`ActorComponent.K2_DestroyComponent` (`self.SM_Gate_Interior_Panel_1077_StaticMeshComponent0`))
          (`ActorComponent.K2_DestroyComponent` (`self.SM_Gate_Interior_Panel_1027_StaticMeshComponent0`))
          (`ActorComponent.K2_DestroyComponent` (`self.SM_Gate_Interior_Panel_993_StaticMeshComponent0`))
          (`ActorComponent.K2_DestroyComponent` (`self.SM_Gate_Interior_Panel_1096_StaticMeshComponent0`))
          (`ActorComponent.K2_DestroyComponent` (`self.SM_Gate_Interior_Panel_1097_StaticMeshComponent0`))
          (`ActorComponent.K2_DestroyComponent` (`self.SM_Gate_Interior_Panel_1158_StaticMeshComponent0`))
          (`ActorComponent.K2_DestroyComponent` (`self.SM_Gate_Interior_Panel_1078_StaticMeshComponent0`))
          (`ActorComponent.K2_DestroyComponent` (`self.SM_Gate_Interior_Panel_1086_StaticMeshComponent0`))
          (`ActorComponent.K2_DestroyComponent` (`self.SM_Gate_Interior_Panel_1084_StaticMeshComponent0`))
          (`ActorComponent.K2_DestroyComponent` (`self.SM_Gate_Interior_Panel_1085_StaticMeshComponent0`))
          (`ActorComponent.K2_DestroyComponent` (`self.SM_Gate_Interior_Panel_1098_StaticMeshComponent0`))
          (`ActorComponent.K2_DestroyComponent` (`self.SM_Gate_Interior_Panel_1154_StaticMeshComponent0`))
          (`ActorComponent.K2_DestroyComponent` (`self.SM_Gate_Interior_Panel_1155_StaticMeshComponent0`))
          (`ActorComponent.K2_DestroyComponent` (`self.SM_Gate_Interior_Panel_1156_StaticMeshComponent0`))
          (`ActorComponent.K2_DestroyComponent` (`self.SM_Gate_Interior_Panel_1090_StaticMeshComponent0`))
          (`ActorComponent.K2_DestroyComponent` (`self.SM_Gate_Interior_Panel_1079_StaticMeshComponent0`))
          (`ActorComponent.K2_DestroyComponent` (`self.SM_Gate_Interior_Panel_1159_StaticMeshComponent0`))
          (`ActorComponent.K2_DestroyComponent` (`self.SM_Gate_Interior_Panel_1081_StaticMeshComponent0`))
          (`ActorComponent.K2_DestroyComponent` (`self.SM_Gate_Interior_Panel_1094_StaticMeshComponent0`))
          (`ActorComponent.K2_DestroyComponent` (`self.SM_Gate_Interior_Panel_1089_StaticMeshComponent0`))
          (`ActorComponent.K2_DestroyComponent` (`self.SM_Gate_Interior_Panel_1095_StaticMeshComponent0`))
          (`ActorComponent.K2_DestroyComponent` (`self.SM_Gate_Interior_Panel_1087_StaticMeshComponent0`))
          (`ActorComponent.K2_DestroyComponent` (`self.SM_Gate_Interior_Panel_1091_StaticMeshComponent0`))
          (`ActorComponent.K2_DestroyComponent` (`self.SM_Gate_Interior_Panel_1080_StaticMeshComponent0`))
          (`ActorComponent.K2_DestroyComponent` (`self.SM_Gate_Interior_Panel_1093_StaticMeshComponent0`))
          (`ActorComponent.K2_DestroyComponent` (`self.SM_Gate_Interior_Panel_1088_StaticMeshComponent0`))
          (`ActorComponent.K2_DestroyComponent` (`self.SM_Gate_Interior_Panel_1083_StaticMeshComponent0`))
          (`ActorComponent.K2_DestroyComponent` (`self.SM_Gate_Interior_Panel_1082_StaticMeshComponent0`))
          (`ActorComponent.K2_DestroyComponent` (`self.SM_Gate_Interior_Panel_1150_StaticMeshComponent0`))
          (`ActorComponent.K2_DestroyComponent` (`self.SM_Gate_Interior_Panel_1147_StaticMeshComponent0`))
          (`ActorComponent.K2_DestroyComponent` (`self.SM_Gate_Interior_Panel_1144_StaticMeshComponent0`))
          (`ActorComponent.K2_DestroyComponent` (`self.SM_Gate_Interior_Panel_1141_StaticMeshComponent0`)))))))
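; BP_SaveInteract is an interactable save point that records the player's respawn transform and writes the save game.
; OnInteract, called from the controller, stores the SavePosition component's world transform and SaveName in the game instance's save object, then saves it.
; A Delay and FlipFlop loop then blinks the point light, with its counter blocking saves while above zero.
; An invalid save object or game instance prints an error.
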(event `self.OnInteract`
  (bind _pointlight (`self.PointLight`))
  (bind _numsaveeffect (`self.NumSaveEffect`))
  ;[1 1 1] Override OnInteract and called from Controller
  (if (<= (`self.NumSaveEffect`) 0)
    (bind _asbp_my_game_instance (cast `/Game/AntizeMenuSystem/Blueprints/BP_MyGameInstance` (`GameplayStatics.GetGameInstance`))
      (:`then`
        (bind _mygamesave (`/Game/AntizeMenuSystem/Blueprints/BP_MyGameInstance.MyGameSave` _asbp_my_game_instance))
        (`/Engine/EditorBlueprintResources/StandardMacros.IsValid` _mygamesave
          (:`Is Valid`
            (set `/Game/AntizeMenuSystem/Blueprints/SaveGame/BP_MySaveGame.PlayerPosition` (`SceneComponent.K2_GetComponentToWorld` (`self.SavePosition`)) _mygamesave)
            (set `/Game/AntizeMenuSystem/Blueprints/SaveGame/BP_MySaveGame.GameName` (`self.SaveName`) _mygamesave)
            (`/Game/AntizeMenuSystem/Blueprints/Function/BP_Antize.SaveGame` _mygamesave)
            ;[1 1 1] Make an effect on save
            (set `self.NumSaveEffect` 0)
            (`KismetSystemLibrary.Delay` 0.05 :!label _label)
            (`/Engine/EditorBlueprintResources/StandardMacros.FlipFlop`
              (:`A`
                (`SceneComponent.SetVisibility` _pointlight true false))
              (:`B`
                (`SceneComponent.SetVisibility` _pointlight false false)))
            (if (<= _numsaveeffect 10)
              (`/Engine/EditorBlueprintResources/StandardMacros.IncrementInt` _numsaveeffect
                (:`  `
                  (goto _label)))
              (else
                (`SceneComponent.SetVisibility` (`self.PointLight`) false false)
                (set `self.NumSaveEffect` 0))))
          (:`Is Not Valid`
            (`KismetSystemLibrary.PrintString` "Error on save, need to join from Main menu"))))
      (:`CastFailed`
        (`KismetSystemLibrary.PrintString` "Error on save, bad game instance")))))

(fn `UserConstructionScript`
  (`parent.UserConstructionScript`))
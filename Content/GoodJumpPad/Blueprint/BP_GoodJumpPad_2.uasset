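; BP_GoodJumpPad_2 is a styled jump pad that launches overlapping characters upward.
; A gravity-scaled square-root formula turns the target height into launch velocity, with a timed DoOnce limiting retriggers.
; Launches play a timeline squash and material pulse plus optional sound, particles and trail; post-process logic is disconnected.
; The construction script applies style mesh and materials, scale, trigger extent, collision per trigger type and a height preview box.
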(event `self.ReceiveTick`
  (params (DeltaSeconds :type "Float (single-precision)")))

(event `self.ReceiveBeginPlay`)

(event `self.Collision Box.OnComponentBeginOverlap`
  (params (OverlappedComponent :type "PrimitiveComponent Object Reference") (OtherActor :type "Actor Object Reference") (OtherComp :type "PrimitiveComponent Object Reference") (OtherBodyIndex :type Integer) (bFromSweep :type Boolean) (SweepResult :type "HitResult Structure (by ref)"))
  (bind _returnvalue (`KismetMathLibrary.MakeTransform` (0.0 0.0 1.0)))
  ;[1 1 1] Trigger Event
  (switch `/Game/GoodJumpPad/Blueprint/Enum/Enum_GJP_TriggerType` (`self.TriggerType`)
    (:`NewEnumerator4`
      _)
    (:`NewEnumerator0`
      _))
  ;[1 1 1] ReTrigger Setting
  (`/Engine/EditorBlueprintResources/StandardMacros.DoOnce` false :!label _label
    (:`Completed`
      ;[1 1 1] End Position Setting
      (bind _ascharacter (cast `Character` OtherActor)
        (:`then`
          (`|ExecutionSequence`
            (:`then_0`
              ;;[1 1 1] Velocity
              (`Character.LaunchCharacter` _ascharacter (`KismetMathLibrary.MakeVector` 0.0 0.0 (`KismetMathLibrary.Sqrt` (+ (`KismetMathLibrary.MultiplyMultiply_FloatFloat` (`KismetMathLibrary.Sqrt` (* (* (+ (* (/ (`MovementComponent.GetGravityZ` (`Character.CharacterMovement` _ascharacter)) -980.0) (`KismetMathLibrary.Abs` (`self.Jump Z Offset End Position`))) 40.0) 2.0) 980.0)) 2.0) 0.0))) (`self.XY Override`) true)
              ;[1 1 1] Jump After
              (`|ExecutionSequence`
                (:`then_0`
                  ;[1 1 1] ReTrigger Setting
                  (`KismetSystemLibrary.Delay` (`self.Event Trigger Interval Seconds Time`) :!label _label_2)
                  (goto _label :!via `Reset`))
                (:`then_1`
                  ;[1 1 1] Add Sound
                  (if (`self.Enable Sound`)
                    (switch `/Game/GoodJumpPad/Blueprint/Enum/Enum_GJP_PadTypes` (`self.GoodJumpPad Style`)
                      (:`NewEnumerator3`
                        (`AddComponent|NODE_AddAudioComponent-6`))
                      (:`NewEnumerator4`
                        (`AddComponent|NODE_AddAudioComponent-5`))
                      (:`NewEnumerator0`
                        (`AddComponent|NODE_AddAudioComponent-1`))
                      (:`NewEnumerator2`
                        (`AddComponent|NODE_AddAudioComponent-4`))
                      (:`NewEnumerator1`
                        (`AddComponent|NODE_AddAudioComponent-3`))
                      (:`NewEnumerator5`
                        (`AddComponent|NODE_AddAudioComponent-2`))
                      (:`NewEnumerator6`
                        (`AddComponent|NODE_AddAudioComponent-7`))
                      (:`NewEnumerator7`
                        (`AddComponent|NODE_AddAudioComponent-9`))))
                  ;[1 1 1] Particle Setting
                  (if (`self.Enable Particle`)
                    (switch `/Game/GoodJumpPad/Blueprint/Enum/Enum_GJP_PadTypes` (`self.GoodJumpPad Style`)
                      (:`NewEnumerator3`
                        (`AddComponent|NODE_AddParticleSystemComponent-0` :`RelativeTransform` _returnvalue))
                      (:`NewEnumerator4`
                        (`AddComponent|NODE_AddParticleSystemComponent-1` :`RelativeTransform` _returnvalue))
                      (:`NewEnumerator0`
                        (`AddComponent|NODE_AddParticleSystemComponent-4` :`RelativeTransform` _returnvalue))
                      (:`NewEnumerator2`
                        (`AddComponent|NODE_AddParticleSystemComponent-3` :`RelativeTransform` _returnvalue))
                      (:`NewEnumerator1`
                        (`AddComponent|NODE_AddParticleSystemComponent-7`))
                      (:`NewEnumerator5`
                        (`AddComponent|NODE_AddParticleSystemComponent-6`))
                      (:`NewEnumerator6`
                        (`AddComponent|NODE_AddParticleSystemComponent-5` :`RelativeTransform` _returnvalue))
                      (:`NewEnumerator7`
                        (`AddComponent|NODE_AddParticleSystemComponent-8` :`RelativeTransform` _returnvalue)))
                    ;[1 1 1] Trail Effect
                    (`AddComponent|NODE_AddParticleSystemComponent-2` :`self` OtherActor)))))
            (:`then_1`
              ;[1 1 1] Pad Scale & Material Effect
              (bind (_direction _effect_intensity _scale_output) (`Timeline|Pad Material Effect TimeLine` :!via `PlayFromStart`)
                (:`Update`
                  (`SceneComponent.SetRelativeScale3D` (`self.Mesh`) (+ (1.0 1.0 1.0) _scale_output))
                  (`MeshComponent.SetScalarParameterValueOnMaterials` (`self.Mesh`) "Effect Intensity" _effect_intensity))))
            (:`then_2`
              ;[1 1 1] Post Process
              (if (`self.Enable Post Process`)
                (if (== OtherActor (`GameplayStatics.GetPlayerCharacter` 0))
                  _)))))
        (:`CastFailed`
          (goto _label_2))))))

(fn `Init`
  (bind _vision_mesh (`self.Vision Mesh`))
  (bind _scale_xy (`self.Scale XY`))
  (bind _returnvalue (+ (`self.Jump Z Offset End Position`) 100.0))
  (`|ExecutionSequence`
    (:`then_0`
      ;[1 1 1] Vision Box Visibility Setting
      (if (`self.Use Vision Box`)
        (`SceneComponent.SetVisibility` _vision_mesh true true)
        (if (`self.Vision Box Show In Game?`)
          (`SceneComponent.SetHiddenInGame` _vision_mesh false true)
          (else
            (`SceneComponent.SetHiddenInGame` _vision_mesh true true)))
        ;[1 1 1] Vision Box Setting
        (`SceneComponent.K2_SetRelativeLocation` (`self.Vision Plane`) (`KismetMathLibrary.MakeVector` 1.0 1.0 _returnvalue) false false)
        (`SceneComponent.K2_SetRelativeLocation` (`self.TextRender`) (`KismetMathLibrary.MakeVector` 1.0 1.0 (+ _returnvalue 40.0)) false false)
        (`SceneComponent.SetRelativeScale3D` (`self.Vision Box`) (`KismetMathLibrary.MakeVector` 1.0 1.0 (+ (/ (`self.Jump Z Offset End Position`) 100.0) 1.0)))
        (`TextRenderComponent.K2_SetText` (`self.TextRender`) (`KismetTextLibrary.Conv_DoubleToText` (`self.Jump Z Offset End Position`) "HalfToEven"))
        (else
          (`SceneComponent.SetVisibility` _vision_mesh false true)
          (set `self.Vision Box Show In Game?` false))))
    (:`then_1`
      (`self.PadTypeSetting`))
    (:`then_2`
      ;[1 1 1] Scale Setting
      (`SceneComponent.SetRelativeScale3D` (`self.DefaultSceneRoot`) (`KismetMathLibrary.MakeVector` _scale_xy _scale_xy _scale_xy)))
    (:`then_3`
      ;[1 1 1] Trigger Collison Box Extent
      (`BoxComponent.SetBoxExtent` (`self.Collision Box`) (`self.Collision Box Extent`) true))
    (:`then_4`
      (switch `/Game/GoodJumpPad/Blueprint/Enum/Enum_GJP_TriggerType` (`self.TriggerType`)
        (:`NewEnumerator4`
          (`PrimitiveComponent.SetCollisionEnabled` (`self.Mesh`) "NoCollision"))
        (:`NewEnumerator0`
          (`PrimitiveComponent.SetCollisionEnabled` (`self.SM_PAD_COLLISION`) "NoCollision"))))))

(fn `PadTypeSetting`
  (bind _mesh (`self.Mesh`))
  ;[1 1 1] Style : Mesh / Material Setting
  (switch `/Game/GoodJumpPad/Blueprint/Enum/Enum_GJP_PadTypes` (`self.GoodJumpPad Style`)
    (:`NewEnumerator3`
      (`StaticMeshComponent.SetStaticMesh` _mesh "/Game/GoodJumpPad/Sources/Props/HighTech/SM_GJP_HighTechPad.SM_GJP_HighTechPad")
      (`PrimitiveComponent.CreateDynamicMaterialInstance` _mesh 0 "/Game/GoodJumpPad/Sources/Props/HighTech/M_GJP_HighTechPad_01.M_GJP_HighTechPad_01" "None")
      (`PrimitiveComponent.CreateDynamicMaterialInstance` _mesh 1 "/Game/GoodJumpPad/Sources/Props/HighTech/M_GJP_HighTechPad_02.M_GJP_HighTechPad_02" "None"))
    (:`NewEnumerator4`
      (`StaticMeshComponent.SetStaticMesh` _mesh "/Game/GoodJumpPad/Sources/Props/Mushroom/SM_GJP_Mushroom.SM_GJP_Mushroom")
      (`PrimitiveComponent.CreateDynamicMaterialInstance` _mesh 0 "/Game/GoodJumpPad/Sources/Props/Mushroom/M_GJP_Mushroom.M_GJP_Mushroom" "None"))
    (:`NewEnumerator0`
      (`StaticMeshComponent.SetStaticMesh` _mesh "/Game/GoodJumpPad/Sources/Props/LotusLeaf/SM_GJP_LotusLeaf.SM_GJP_LotusLeaf")
      (`PrimitiveComponent.CreateDynamicMaterialInstance` _mesh 0 "/Game/GoodJumpPad/Sources/Props/LotusLeaf/M_GJP_LotusLeaf.M_GJP_LotusLeaf" "None"))
    (:`NewEnumerator2`
      (`StaticMeshComponent.SetStaticMesh` _mesh "/Game/GoodJumpPad/Sources/Props/TurtleShell/SM_GJP_TurleShell.SM_GJP_TurleShell")
      (`PrimitiveComponent.CreateDynamicMaterialInstance` _mesh 0 "/Game/GoodJumpPad/Sources/Props/TurtleShell/M_GJP_TurleShell.M_GJP_TurleShell" "None"))
    (:`NewEnumerator1`
      (`StaticMeshComponent.SetStaticMesh` _mesh "/Game/GoodJumpPad/Sources/Props/Springs/SM_GJP_Springs.SM_GJP_Springs")
      (`PrimitiveComponent.CreateDynamicMaterialInstance` _mesh 0 "/Game/GoodJumpPad/Sources/Props/Springs/M_GJP_Springs.M_GJP_Springs" "None"))
    (:`NewEnumerator5`
      (`StaticMeshComponent.SetStaticMesh` _mesh "/Game/GoodJumpPad/Sources/Props/Tires/SM_GJP_Tires.SM_GJP_Tires")
      (`PrimitiveComponent.CreateDynamicMaterialInstance` _mesh 0 "/Game/GoodJumpPad/Sources/Props/Tires/M_GJP_Tires.M_GJP_Tires" "None"))
    (:`NewEnumerator6`
      (`StaticMeshComponent.SetStaticMesh` _mesh "/Game/GoodJumpPad/Sources/Props/Stool/SM_GJP_Stool.SM_GJP_Stool")
      (`PrimitiveComponent.CreateDynamicMaterialInstance` _mesh 0 "/Game/GoodJumpPad/Sources/Props/Stool/M_GJP_Stool.M_GJP_Stool" "None"))
    (:`NewEnumerator7`
      (`StaticMeshComponent.SetStaticMesh` _mesh "/Game/Assets/Meshes/Cupcake.Cupcake")
      (`PrimitiveComponent.CreateDynamicMaterialInstance` _mesh 1 "/Game/AdvancedPuzzleConstructor/Materials/Weapons/MI_TelekenesisGunLight.MI_TelekenesisGunLight" "None")
      (`PrimitiveComponent.CreateDynamicMaterialInstance` _mesh 0 "/Game/Assets/Materials/CaliperPaint/MI_Caliper_Yellow.MI_Caliper_Yellow" "None")
      (`PrimitiveComponent.CreateDynamicMaterialInstance` _mesh 2 "/Game/MadMeshes/DynamicSlideshow/Materials/MI_FlatBlack.MI_FlatBlack" "None"))))

(fn `UserConstructionScript`
  (`self.Init`))